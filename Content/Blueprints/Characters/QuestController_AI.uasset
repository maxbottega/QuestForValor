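; AI controller for quest characters that runs the pawn's behavior tree and handles target acquisition.
; On possess it copies faction data and seeds the blackboard with spawn, patrol and health values.
; PawnSensing sight and hearing pick targets by faction standing, or borrow a sensed same-faction ally's target.
; Setter functions push target, follow, state and combat flags to the blackboard; the scripted-state check always passes as not scripted.
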(event OnSeePawn(PawnSensing)
  (params (Pawn :type Pawn%20Object%20Reference))
  ;[1 1 1] AI has seen/heard something
  (AI|CheckSensedPawnforTarget Pawn))

(event OnHearNoise(PawnSensing)
  (params (Instigator :type Pawn%20Object%20Reference) (Location :type Vector%20%28by%20ref%29 :default "0, 0, 0") (Volume :type Float%20%28single-precision%29))
  ;[1 1 1] AI has seen/heard something
  (AI|CheckSensedPawnforTarget Instigator))

(event EventAssignPatrolPath
  (params (New%20Patrol%20Path :type Quest%20Patrol%20Path%20Object%20Reference))
  ;[1 1 1] Set patrol path
  (AI|SetPatrolPath New%20Patrol%20Path))

(event EventOnPossess
  (params (PossessedPawn :type Pawn%20Object%20Reference))
  ;[1 1 1] Reference to controlled character
  (bind _asquest_character_ai (Utilities|Casting|CastToQuestCharacter_AI PossessedPawn))
  (Variables|AI|SetAICharacter _asquest_character_ai)
  ;[1 1 1] Set the faction and standing
  (Variables|AI|SetAIFaction (Variables|/Game/Blueprints/Characters/QuestCharacter.QuestCharacter_C|GetCharacterFaction (Variables|AI|GetAICharacter)))
  (Variables|AI|SetFactionStanding (Variables|/Game/Blueprints/Characters/QuestCharacter.QuestCharacter_C|GetFactionStanding (Variables|AI|GetAICharacter)))
  ;[1 1 1] Set the blackboard and behavior tree
  (Class|AIController|UseBlackboard "/Game/AI/BBD_EnemyAI.BBD_EnemyAI")
  (AI|RunBehaviorTree (Variables|/Game/Blueprints/Characters/QuestCharacter_AI.QuestCharacter_AI_C|GetBehaviorTree (Variables|AI|GetAICharacter)))
  ;[1 1 1] Spawn
  (AI|SetCharacterSpawning (Variables|/Game/Blueprints/Characters/QuestCharacter.QuestCharacter_C|GetBeginWithSpawnAnim (Variables|AI|GetAICharacter)))
  ;[1 1 1] Set the initial patrol path
  (Utilities|IsValid (Variables|AI|GetPatrolPath)
    (:Is%20Valid
      (AI|SetPatrolPath (Variables|AI|GetPatrolPath)))
    (:Is%20Not%20Valid
      _))
  ;[1 1 1] Set health
  (AI|SetCharacterHealthScalar (/ (Variables|/Game/Blueprints/Characters/QuestCharacter.QuestCharacter_C|GetHealth (Variables|AI|GetAICharacter)) (Variables|/Game/Blueprints/Characters/QuestCharacter.QuestCharacter_C|GetMaxHealth (Variables|AI|GetAICharacter)))))

(fn ConstructionScript)

(fn SetCurrentTarget
  (params (NewTarget :type Actor%20Object%20Reference))
  ;[1 1 1] Init vars
  (LocalVariables|SetNewTargetLocal NewTarget)
  ;[1 1 1] Only if our new target isn't the old one we have
  (if (!= (LocalVariables|GetNewTargetLocal) (Variables|AI|GetCurrentTarget))
    ;[1 1 1] Check if everything is ok
    (Variables|AI|SetCurrentTarget (LocalVariables|GetNewTargetLocal))
    (Utilities|IsValid (AI|GetBlackboard self)
      (:Is%20Valid
        ;[1 1 1] Acquire the actor as a target
        (Default|SetLockonTarget (Variables|AI|GetAICharacter) (Variables|AI|GetCurrentTarget))
        ;[1 1 1] Set state, blackboard values and walk speed
        (AI|Components|Blackboard|SetValueasObject (AI|GetBlackboard self) (Utilities|Name|MakeLiteralName "CurrentTarget") (Variables|AI|GetCurrentTarget))))))

(fn SetPatrolPath
  (params (NewPatrolPath :type Quest%20Patrol%20Path%20Object%20Reference))
  ;[1 1 1] Make sure there's a new patrol being provided
  (bind _output_get (LocalVariables|SetNewPatrolPathLocal NewPatrolPath))
  (bind _output_get_2 (Variables|AI|SetPatrolPath _output_get))
  (Utilities|IsValid _output_get_2
    (:Is%20Valid
      ;[1 1 1] Has the behavior tree been initialized yet?
      (Utilities|IsValid (AI|GetBlackboard self)
        (:Is%20Valid
          ;[1 1 1] Send the info to the blackboard and set a new state
          (AI|Components|Blackboard|SetValueasObject (AI|GetBlackboard self) (Utilities|Name|MakeLiteralName "PatrolPath") (Variables|AI|GetPatrolPath))
          (AI|SetFinishedPatrolPath false))))))

(fn SetGlobalActionCooldown
  (params (NewGlobalActionCooldown :type Float%20%28single-precision%29 :default 0.0))
  (bind _self self)
  (bind _returnvalue (AI|GetBlackboard _self))
  (LocalVariables|SetNewGlobalActionCooldownLocal NewGlobalActionCooldown)
  (Utilities|IsValid _returnvalue
    (:Is%20Valid
      (AI|Components|Blackboard|SetValueasFloat _returnvalue (Utilities|Name|MakeLiteralName "GlobalActionCooldown") (LocalVariables|GetNewGlobalActionCooldownLocal)))))

(fn SetAIState
  (params (NewState :type Enum_AIState%20Enum))
  ;[1 1 1] Update the var
  (LocalVariables|SetAIStateLocal NewState)
  ;[1 1 1] Update the blackboard
  (AI|Components|Blackboard|SetValueasEnum (AI|GetBlackboard self) (Utilities|Name|MakeLiteralName "AIState") (LocalVariables|GetAIStateLocal))
  ;[1 1 1] If we just entered scripted, clear our target
  (switch Utilities|FlowControl|Switch|SwitchonEnum_AIState (LocalVariables|GetAIStateLocal)
    (:NewEnumerator0
      (AI|SetCanTarget true))
    (:NewEnumerator3
      (AI|SetCanTarget false)
      (AI|SetCurrentTarget)
      (Default|ClearLockonTarget (Variables|AI|GetAICharacter)))))

(fn CheckTargetFactionStanding
  (params (Pawn :type Pawn%20Object%20Reference))
  (bind _output_get (LocalVariables|SetPawnLocal Pawn))
  (bind _asquest_character (Utilities|Casting|CastToQuestCharacter _output_get))
  (LocalVariables|SetQuestCharacterLocal _asquest_character)
  (return (Utilities|Array|ContainsItem (Variables|AI|GetFactionStanding) (Utilities|Struct|MakeStruct_FactionStanding (Variables|/Game/Blueprints/Characters/QuestCharacter.QuestCharacter_C|GetCharacterFaction (LocalVariables|GetQuestCharacterLocal)) "NewEnumerator0"))))

(fn CheckAllyforCurrentTarget
  (params (Pawn :type Pawn%20Object%20Reference))
  (bind _asquest_character_ai (Utilities|Casting|CastToQuestCharacter_AI Pawn))
  (if (Utilities|Enum|Equal(Enum) (Variables|/Game/Blueprints/Characters/QuestCharacter.QuestCharacter_C|GetCharacterFaction _asquest_character_ai) (Variables|AI|GetAIFaction))
    (bind _asquest_controller_ai (Utilities|Casting|CastToQuestController_AI (Pawn|GetController _asquest_character_ai)))
    (Utilities|IsValid (Variables|QuestController_AI_C|GetCurrentTarget _asquest_controller_ai)
      (:Is%20Valid
        (AI|SetCurrentTarget (Variables|QuestController_AI_C|GetCurrentTarget _asquest_controller_ai))))))

(fn CheckSensedPawnforTarget
  (params (SensedPawn :type Pawn%20Object%20Reference))
  ;[1 1 1] Init var
  (bind _asquest_character (Utilities|Casting|CastToQuestCharacter SensedPawn))
  (LocalVariables|SetSensedPawnLocal _asquest_character)
  ;[1 1 1] Can we target?
  (if (Variables|AI|GetCanTarget)
    ;[1 1 1] Are we not scripted?
    (Utilities|CheckAIScriptedState
      (:NotScripted
        ;[1 1 1] Make sure the pawn is not dead
        (bind _isalive (Default|GetIsAlive (LocalVariables|GetSensedPawnLocal)))
        (if _isalive
          ;[1 1 1] Make sure they are targetable
          (bind _istargetable (Default|GetIsTargetable (LocalVariables|GetSensedPawnLocal)))
          (if _istargetable
            ;[1 1 1] Do we not have a target?
            (Utilities|IsValid (Variables|AI|GetCurrentTarget)
              (:Is%20Not%20Valid
                ;[1 1 1] Friend or foe?
                (bind _pawnisenemy (AI|CheckTargetFactionStanding (LocalVariables|GetSensedPawnLocal)))
                (if _pawnisenemy
                  ;[1 1 1] Found a target
                  (AI|SetCurrentTarget (LocalVariables|GetSensedPawnLocal))
                  ;[1 1 1] Let everyone know!
                  (Default|CallFoundNewTarget (LocalVariables|GetSensedPawnLocal))
                  (else
                    ;[1 1 1] Check if our friends have a target
                    (AI|CheckAllyforCurrentTarget (LocalVariables|GetSensedPawnLocal))))))))))))

(fn ClearCurrentTarget
  ;[1 1 1] Clear the vars
  (Variables|AI|SetCurrentTarget 0)
  (Variables|/Game/Blueprints/Characters/QuestCharacter.QuestCharacter_C|SetCurrentTarget (Variables|AI|GetAICharacter) 0)
  (AI|Components|Blackboard|SetValueasObject (AI|GetBlackboard self) (Utilities|Name|MakeLiteralName "CurrentTarget") 0))

(fn GetCurrentTarget
  (return (Variables|AI|GetCurrentTarget)))

(fn SetCanTarget
  (params (CanTarget :type Boolean :default false))
  (bind _output_get (Variables|AI|SetCanTarget CanTarget))
  (if (not _output_get)
    (AI|ClearCurrentTarget)))

(fn GetCanTarget
  (return (Variables|AI|GetCanTarget)))

(fn SetFollowTarget
  (params (FollowTarget :type Actor%20Object%20Reference))
  ;[1 1 1] Init var
  (bind _output_get (LocalVariables|SetFollowTargetLocal FollowTarget))
  ;[1 1 1] Set our var for the entire class
  (Variables|AI|SetFollowTarget _output_get)
  ;[1 1 1] Send it to the blackboard
  (AI|Components|Blackboard|SetValueasObject (AI|GetBlackboard self) (Utilities|Name|MakeLiteralName "FollowTarget") (Variables|AI|GetFollowTarget)))

(fn ClearFollowTarget
  (Variables|AI|SetFollowTarget 0)
  ;[1 1 1] Send it to the blackboard
  (AI|Components|Blackboard|SetValueasObject (AI|GetBlackboard self) (Utilities|Name|MakeLiteralName "FollowTarget") 0))

(fn SetCharacterDead
  (params (IsDead :type Boolean))
  (AI|Components|Blackboard|SetValueasBool (AI|GetBlackboard self) (Utilities|Name|MakeLiteralName "IsDead") IsDead))

(fn SetCharacterHit
  (params (IsHit :type Boolean))
  (AI|Components|Blackboard|SetValueasBool (AI|GetBlackboard self) (Utilities|Name|MakeLiteralName "IsHit") IsHit))

(fn SetCharacterSpawning
  (params (IsSpawning :type Boolean))
  (AI|Components|Blackboard|SetValueasBool (AI|GetBlackboard self) (Utilities|Name|MakeLiteralName "IsSpawning") IsSpawning)
  (bind _asquest_character_ai (Utilities|Casting|CastToQuestCharacter_AI (Pawn|GetControlledPawn)))
  (Variables|/Game/Blueprints/Characters/QuestCharacter.QuestCharacter_C|SetIsSpawning _asquest_character_ai IsSpawning))

(fn SetCharacterHealthScalar
  (params (HealthScalar :type Float%20%28single-precision%29))
  (AI|Components|Blackboard|SetValueasFloat (AI|GetBlackboard self) (Utilities|Name|MakeLiteralName "HealthScalar") HealthScalar))

(fn SetHasAttackToken
  (params (HasAttackToken :type Boolean))
  (AI|Components|Blackboard|SetValueasBool (AI|GetBlackboard self) (Utilities|Name|MakeLiteralName "HasAttackToken") HasAttackToken))

(fn SetSightRadius
  (params (SightRadius :type Float%20%28single-precision%29))
  (Variables|/Script/AIModule.PawnSensingComponent|SetSightRadius (Variables|Default|GetPawnSensing) SightRadius))

(fn SetFinishedPatrolPath
  (params (BoolValue :type Boolean))
  (AI|Components|Blackboard|SetValueasBool (AI|GetBlackboard self) (Utilities|Name|MakeLiteralName "FinishedPatrolPath") BoolValue)
  (return))