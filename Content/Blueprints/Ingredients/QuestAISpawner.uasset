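; Placeable spawner that creates one quest AI character on begin play or when Juno enters its radius or trigger box, per SpawnType.
; The construction script maps the chosen character class through a cast chain to a behavior tree and editor preview mesh, showing a billboard if none matches.
; SpawnAI runs once, adds the controller to a named game-state squad, assigns any patrol path, and stores references for GetSpawnedAI.
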(event OnActorBeginOverlap(SpawnTriggerBox)
  (params (OtherActor :type Actor%20Object%20Reference))
  ;[1 1 1] Spawn from trigger box
  (Utilities|Casting|CastToQuestCharacter_Juno OtherActor)
  (switch Utilities|FlowControl|Switch|SwitchonEnum_SpawnerTypes (Variables|AISpawner|GetSpawnType)
    (:NewEnumerator1
      ;[1 1 1] Spawn the AI and give them a patrol path if one is supplied
      (Utilities|FlowControl|DoOnce false
        (:Completed
          (CallFunction|SpawnAI))))))

(event OnComponentBeginOverlap(SpawnRadiusSphere)
  (params (OtherActor :type Actor%20Object%20Reference) (OtherComp :type Primitive%20Component%20Object%20Reference) (OtherBodyIndex :type Integer) (bFromSweep :type Boolean) (SweepResult :type Hit%20Result%20Structure%20%28by%20ref%29))
  ;[1 1 1] Spawn from entering a radius
  (Utilities|Casting|CastToQuestCharacter_Juno OtherActor)
  (switch Utilities|FlowControl|Switch|SwitchonEnum_SpawnerTypes (Variables|AISpawner|GetSpawnType)
    (:NewEnumerator2
      ;[1 1 1] Spawn the AI and give them a patrol path if one is supplied
      (Utilities|FlowControl|DoOnce false
        (:Completed
          (CallFunction|SpawnAI))))))

(event EventBeginPlay
  ;[1 1 1] Destroy the preview mesh
  (Components|DestroyComponent (Variables|Default|GetPreviewMesh))
  ;[1 1 1] Spawn from begin play
  (switch Utilities|FlowControl|Switch|SwitchonEnum_SpawnerTypes (Variables|AISpawner|GetSpawnType)
    (:NewEnumerator0
      ;[1 1 1] Spawn the AI and give them a patrol path if one is supplied
      (Utilities|FlowControl|DoOnce false
        (:Completed
          (CallFunction|SpawnAI))))))

(fn ConstructionScript
  (bind _spawnradiussphere (Variables|Default|GetSpawnRadiusSphere))
  ;[1 1 1] Set the size of the radius trigger event
  (if (Utilities|Enum|Equal(Enum) (Variables|AISpawner|GetSpawnType) "NewEnumerator2")
    (Rendering|SetVisibility _spawnradiussphere true false)
    (Components|Sphere|SetSphereRadius (Variables|Default|GetSpawnRadiusSphere) (Variables|AISpawner|GetSpawnRadius) false)
    (else
      (Rendering|SetVisibility _spawnradiussphere false false)))
  ;[1 1 1] Rotate and scale the preview mesh
  (Transformation|SetRelativeRotation (Variables|Default|GetPreviewMesh) "0,270.000000, 0" false false)
  (Transformation|SetWorldScale3D (Variables|Default|GetPreviewMesh) (Variables|AISpawner|GetPreviewMeshScale))
  ;[1 1 1] Skeletons
  (Utilities|Casting|CastToQuestCharacter_AI_SkeletonArcherClass (Variables|AISpawner|GetCharacterToSpawn)
    (:then
      (Variables|AISpawner|SetMeshToUse "/Game/Characters/SkeletonArcher/Meshes/SkeletonArcher_SkeletalMesh.SkeletonArcher_SkeletalMesh")
      (Variables|AISpawner|SetBehaviorTree "/Game/AI/BT_SkeletonArcher.BT_SkeletonArcher")
      ;[1 1 1] Set the preview mesh
      (Class|SkinnedMeshComponent|SetSkeletalMesh (Variables|Default|GetPreviewMesh) (Variables|AISpawner|GetMeshToUse) :!label _label)
      ;[1 1 1] Hide the billboard since it displays a character
      (Rendering|SetVisibility (Variables|Default|GetSpawnerBillboard) false false))
    (:CastFailed
      (Utilities|Casting|CastToQuestCharacter_AI_SkeletonGruntClass (Variables|AISpawner|GetCharacterToSpawn)
        (:then
          (Variables|AISpawner|SetMeshToUse "/Game/Characters/SkeletonGrunt/Meshes/SkeletonGrunt_SkeletalMesh.SkeletonGrunt_SkeletalMesh")
          (Variables|AISpawner|SetBehaviorTree "/Game/AI/BT_SkeletonGrunt.BT_SkeletonGrunt")
          (goto _label))
        (:CastFailed
          (Utilities|Casting|CastToQuestCharacter_AI_SkeletonKingClass (Variables|AISpawner|GetCharacterToSpawn)
            (:then
              (Variables|AISpawner|SetMeshToUse "/Game/Characters/SkeletonKing/Meshes/SkeletonKing_SkeletalMesh.SkeletonKing_SkeletalMesh")
              (Variables|AISpawner|SetBehaviorTree "/Game/AI/BT_SkeletonKing.BT_SkeletonKing")
              (goto _label))
            (:CastFailed
              (Utilities|Casting|CastToQuestCharacter_AI_SkeletonMageClass (Variables|AISpawner|GetCharacterToSpawn)
                (:then
                  (Variables|AISpawner|SetMeshToUse "/Game/Characters/SkeletonMage/Meshes/SkeletonMage_SkeletalMesh.SkeletonMage_SkeletalMesh")
                  (Variables|AISpawner|SetBehaviorTree "/Game/AI/BT_SkeletonMage.BT_SkeletonMage")
                  (goto _label))
                (:CastFailed
                  (Utilities|Casting|CastToQuestCharacter_AI_SkeletonSwordsmanClass (Variables|AISpawner|GetCharacterToSpawn)
                    (:then
                      (Variables|AISpawner|SetMeshToUse "/Game/Characters/SkeletonSwordsman/Meshes/SkeletonSwordsman_SkeletalMesh.SkeletonSwordsman_SkeletalMesh")
                      (Variables|AISpawner|SetBehaviorTree "/Game/AI/BT_SkeletonSwordsman.BT_SkeletonSwordsman")
                      (goto _label))
                    (:CastFailed
                      ;[1 1 1] Human
                      (Utilities|Casting|CastToQuestCharacter_AI_HumanArcherClass (Variables|AISpawner|GetCharacterToSpawn)
                        (:then
                          (Variables|AISpawner|SetMeshToUse "/Game/Characters/HumanArcher/Meshes/HumanArcher_SkeletalMesh.HumanArcher_SkeletalMesh")
                          (Variables|AISpawner|SetBehaviorTree "/Game/AI/BT_HumanArcher.BT_HumanArcher")
                          (goto _label))
                        (:CastFailed
                          (Utilities|Casting|CastToQuestCharacter_AI_HumanWarriorClass (Variables|AISpawner|GetCharacterToSpawn)
                            (:then
                              (Variables|AISpawner|SetMeshToUse "/Game/Characters/HumanWarrior/Meshes/HumanWarrior_SkeletalMesh.HumanWarrior_SkeletalMesh")
                              (Variables|AISpawner|SetBehaviorTree "/Game/AI/BT_HumanWarrior.BT_HumanWarrior")
                              (goto _label))
                            (:CastFailed
                              (Utilities|Casting|CastToQuestCharacter_AI_HumanWorkerClass (Variables|AISpawner|GetCharacterToSpawn)
                                (:then
                                  (Variables|AISpawner|SetMeshToUse "/Game/Characters/HumanWorker/Meshes/HumanWorker_SkeletalMesh.HumanWorker_SkeletalMesh")
                                  (Variables|AISpawner|SetBehaviorTree "/Game/AI/BT_HumanWorker.BT_HumanWorker")
                                  (goto _label))
                                (:CastFailed
                                  ;[1 1 1] Animals
                                  (Utilities|Casting|CastToQuestCharacter_AI_AnimalCatClass (Variables|AISpawner|GetCharacterToSpawn)
                                    (:then
                                      (Variables|AISpawner|SetMeshToUse "/Game/Characters/AnimalCat/Meshes/AnimalCat_SkeletalMesh.AnimalCat_SkeletalMesh")
                                      (Variables|AISpawner|SetBehaviorTree "/Game/AI/BT_AnimalCat.BT_AnimalCat")
                                      (goto _label))
                                    (:CastFailed
                                      (Utilities|Casting|CastToQuestCharacter_AI_AnimalCowClass (Variables|AISpawner|GetCharacterToSpawn)
                                        (:then
                                          (Variables|AISpawner|SetMeshToUse "/Game/Characters/AnimalCow/Meshes/AnimalCow_SkeletalMesh.AnimalCow_SkeletalMesh")
                                          (Variables|AISpawner|SetBehaviorTree "/Game/AI/BT_AnimalCow.BT_AnimalCow")
                                          (goto _label))
                                        (:CastFailed
                                          (Utilities|Casting|CastToQuestCharacter_AI_AnimalPigClass (Variables|AISpawner|GetCharacterToSpawn)
                                            (:then
                                              (Variables|AISpawner|SetMeshToUse "/Game/Characters/AnimalPig/Meshes/AnimalPig_SkeletalMesh.AnimalPig_SkeletalMesh")
                                              (Variables|AISpawner|SetBehaviorTree "/Game/AI/BT_AnimalPig.BT_AnimalPig")
                                              (goto _label))
                                            (:CastFailed
                                              (Utilities|Casting|CastToQuestCharacter_AI_AnimalRoosterClass (Variables|AISpawner|GetCharacterToSpawn)
                                                (:then
                                                  (Variables|AISpawner|SetMeshToUse "/Game/Characters/AnimalRooster/Meshes/AnimalRooster_SkeletalMesh.AnimalRooster_SkeletalMesh")
                                                  (Variables|AISpawner|SetBehaviorTree "/Game/AI/BT_AnimalRooster.BT_AnimalRooster")
                                                  (goto _label))
                                                (:CastFailed
                                                  ;[1 1 1] Micro
                                                  (Utilities|Casting|CastToQuestCharacter_AI_MicroDemonClass (Variables|AISpawner|GetCharacterToSpawn)
                                                    (:then
                                                      (Variables|AISpawner|SetMeshToUse "/Game/Characters/MicroDemon/Meshes/MicroDemon_SkeletalMesh.MicroDemon_SkeletalMesh")
                                                      (Variables|AISpawner|SetBehaviorTree "/Game/AI/BT_MicroDemon.BT_MicroDemon")
                                                      (goto _label))
                                                    (:CastFailed
                                                      (Utilities|Casting|CastToQuestCharacter_AI_MicroDragonClass (Variables|AISpawner|GetCharacterToSpawn)
                                                        (:then
                                                          (Variables|AISpawner|SetMeshToUse "/Game/Characters/MicroDragon/Meshes/MicroDragon_SkeletalMesh.MicroDragon_SkeletalMesh")
                                                          (Variables|AISpawner|SetBehaviorTree "/Game/AI/BT_MicroDragon.BT_MicroDragon")
                                                          (goto _label))
                                                        (:CastFailed
                                                          ;[1 1 1] Mini
                                                          (Utilities|Casting|CastToQuestCharacter_AI_MiniDragonClass (Variables|AISpawner|GetCharacterToSpawn)
                                                            (:then
                                                              (Variables|AISpawner|SetMeshToUse "/Game/Characters/MiniDragon/Meshes/MiniDragon_SkeletalMesh.MiniDragon_SkeletalMesh")
                                                              (Variables|AISpawner|SetBehaviorTree "/Game/AI/BT_MiniDragon.BT_MiniDragon")
                                                              (goto _label))
                                                            (:CastFailed
                                                              ;[1 1 1] Demons
                                                              (Utilities|Casting|CastToQuestCharacter_AI_DemonBombClass (Variables|AISpawner|GetCharacterToSpawn)
                                                                (:then
                                                                  (Variables|AISpawner|SetMeshToUse "/Game/Characters/DemonBomb/Meshes/DemonBomb_SkeletalMesh.DemonBomb_SkeletalMesh")
                                                                  (Variables|AISpawner|SetBehaviorTree "/Game/AI/BT_DemonBomb.BT_DemonBomb")
                                                                  (goto _label))
                                                                (:CastFailed
                                                                  (Utilities|Casting|CastToQuestCharacter_AI_DemonBossClass (Variables|AISpawner|GetCharacterToSpawn)
                                                                    (:then
                                                                      (Variables|AISpawner|SetMeshToUse "/Game/Characters/DemonBoss/Meshes/DemonBoss_SkeletalMesh.DemonBoss_SkeletalMesh")
                                                                      (Variables|AISpawner|SetBehaviorTree "/Game/AI/BT_DemonBoss.BT_DemonBoss")
                                                                      (goto _label))
                                                                    (:CastFailed
                                                                      (Utilities|Casting|CastToQuestCharacter_AI_DemonFatClass (Variables|AISpawner|GetCharacterToSpawn)
                                                                        (:then
                                                                          (Variables|AISpawner|SetMeshToUse "/Game/Characters/DemonFat/Meshes/DemonFat_SkeletalMesh.DemonFat_SkeletalMesh")
                                                                          (Variables|AISpawner|SetBehaviorTree "/Game/AI/BT_DemonFat.BT_DemonFat")
                                                                          (goto _label))
                                                                        (:CastFailed
                                                                          (Utilities|Casting|CastToQuestCharacter_AI_DemonGruntClass (Variables|AISpawner|GetCharacterToSpawn)
                                                                            (:then
                                                                              (Variables|AISpawner|SetMeshToUse "/Game/Characters/DemonGrunt/Meshes/DemonGrunt_SkeletalMesh.DemonGrunt_SkeletalMesh")
                                                                              (Variables|AISpawner|SetBehaviorTree "/Game/AI/BT_DemonGrunt.BT_DemonGrunt")
                                                                              (goto _label))
                                                                            (:CastFailed
                                                                              (Utilities|Casting|CastToQuestCharacter_AI_DemonImpClass (Variables|AISpawner|GetCharacterToSpawn)
                                                                                (:then
                                                                                  (Variables|AISpawner|SetMeshToUse "/Game/Characters/DemonImp/Meshes/DemonImp_SkeletalMesh.DemonImp_SkeletalMesh")
                                                                                  (Variables|AISpawner|SetBehaviorTree "/Game/AI/BT_DemonImp.BT_DemonImp")
                                                                                  (goto _label))
                                                                                (:CastFailed
                                                                                  ;[1 1 1] Zombies
                                                                                  (Utilities|Casting|CastToQuestCharacter_AI_ZombieBossClass (Variables|AISpawner|GetCharacterToSpawn)
                                                                                    (:then
                                                                                      (Variables|AISpawner|SetMeshToUse "/Game/Characters/ZombieBoss/Meshes/ZombieBoss_SkeletalMesh.ZombieBoss_SkeletalMesh")
                                                                                      (Variables|AISpawner|SetBehaviorTree "/Game/AI/BT_ZombieBoss.BT_ZombieBoss")
                                                                                      (goto _label))
                                                                                    (:CastFailed
                                                                                      (Utilities|Casting|CastToQuestCharacter_AI_ZombieCommonerClass (Variables|AISpawner|GetCharacterToSpawn)
                                                                                        (:then
                                                                                          (Variables|AISpawner|SetMeshToUse "/Game/Characters/ZombieCommoner/Meshes/ZombieCommoner_SkeletalMesh.ZombieCommoner_SkeletalMesh")
                                                                                          (Variables|AISpawner|SetBehaviorTree "/Game/AI/BT_ZombieCommoner.BT_ZombieCommoner")
                                                                                          (goto _label))
                                                                                        (:CastFailed
                                                                                          (Utilities|Casting|CastToQuestCharacter_AI_ZombieFatClass (Variables|AISpawner|GetCharacterToSpawn)
                                                                                            (:then
                                                                                              (Variables|AISpawner|SetMeshToUse "/Game/Characters/ZombieFat/Meshes/ZombieFat_SkeletalMesh.ZombieFat_SkeletalMesh")
                                                                                              (Variables|AISpawner|SetBehaviorTree "/Game/AI/BT_ZombieFat.BT_ZombieFat")
                                                                                              (goto _label))
                                                                                            (:CastFailed
                                                                                              (Utilities|Casting|CastToQuestCharacter_AI_ZombieMurdererClass (Variables|AISpawner|GetCharacterToSpawn)
                                                                                                (:then
                                                                                                  (Variables|AISpawner|SetMeshToUse "/Game/Characters/ZombieMurderer/Meshes/ZombieMurderer_SkeletalMesh.ZombieMurderer_SkeletalMesh")
                                                                                                  (Variables|AISpawner|SetBehaviorTree "/Game/AI/BT_ZombieMurderer.BT_ZombieMurderer")
                                                                                                  (goto _label))
                                                                                                (:CastFailed
                                                                                                  (Utilities|Casting|CastToQuestCharacter_AI_ZombieSnapperClass (Variables|AISpawner|GetCharacterToSpawn)
                                                                                                    (:then
                                                                                                      (Variables|AISpawner|SetMeshToUse "/Game/Characters/ZombieSnapper/Meshes/ZombieSnapper_SkeletalMesh.ZombieSnapper_SkeletalMesh")
                                                                                                      (Variables|AISpawner|SetBehaviorTree "/Game/AI/BT_ZombieSnapper.BT_ZombieSnapper")
                                                                                                      (goto _label))
                                                                                                    (:CastFailed
                                                                                                      ;[1 1 1] Show the billboard if no valid character is selected
                                                                                                      (Rendering|SetVisibility (Variables|Default|GetSpawnerBillboard) true false))))))))))))))))))))))))))))))))))))))))))))))))))))

(fn SpawnAI
  (bind _spawnpoint (Variables|Default|GetSpawnPoint))
  (bind _initialpatrolpath (Variables|AISpawner|GetInitialPatrolPath))
  ;[1 1 1] Spawn the AI
  (bind _returnvalue (AI|SpawnAIFromClass (Variables|AISpawner|GetCharacterToSpawn) (Variables|AISpawner|GetBehaviorTree) (Transformation|GetWorldLocation _spawnpoint) (Transformation|GetWorldRotation _spawnpoint) true))
  ;[1 1 1] Set the local vars
  (Variables|AISpawner|SetCharacter (.AsQuest%20Character%20AI (Utilities|Casting|CastToQuestCharacter_AI _returnvalue)))
  (Variables|AISpawner|SetController (.AsQuest%20Controller%20AI (Utilities|Casting|CastToQuestController_AI (Pawn|GetController (.AsQuest%20Character%20AI (Utilities|Casting|CastToQuestCharacter_AI _returnvalue))))))
  (Default|AddtoSquad (.AsQuest%20Game%20State (Utilities|Casting|CastToQuestGameState (Game|GetGameState))) (Variables|AISpawner|GetSquadName) (Variables|AISpawner|GetController))
  ;[1 1 1] Give them a patrol if there is one
  (Utilities|IsValid _initialpatrolpath
    (:Is%20Valid
      (Default|AssignPatrolPath (Variables|AISpawner|GetController) _initialpatrolpath))
    (:Is%20Not%20Valid
      _))
  ;[1 1 1] Return
  (return (Variables|AISpawner|GetCharacter) (Variables|AISpawner|GetController)))

(fn GetSpawnedAI
  ;[1 1 1] Check if the character is valid
  (Utilities|IsValid (Variables|AISpawner|GetCharacter)
    (:Is%20Valid
      ;[1 1 1] Check if the controller is valid
      (Utilities|IsValid (Variables|AISpawner|GetController)
        (:Is%20Valid
          (return (Variables|AISpawner|GetCharacter) (Variables|AISpawner|GetController)))
        (:Is%20Not%20Valid
          (Development|PrintString "WARNING: Attempting to get spawned AI while there is no valid controller"))))
    (:Is%20Not%20Valid
      (Development|PrintString "WARNING: Attempting to get spawned AI while there is no valid character"))))