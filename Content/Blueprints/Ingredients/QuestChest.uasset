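; Quest chest actor that opens once and can spawn a quest pickup (potion, key or gold settings) at its arrow.
; Construction picks meshes, padlock and hinge offset from the chest type, parents the lid to the hinge, and sets the starting highlight.
; Player interaction respects the lock, while OpenChest bypasses it; both run a timeline that rotates the lid.
; When opening finishes, it broadcasts whether the player opened it and any spawned pickup.
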(event Custom|OpenChest
  ;[1 1 1] Interact or event is called
  ;[1 1 1] Check if locked
  (Variables|Chest|SetPlayerInteracted false)
  ;[1 1 1] Make sure to check if it hasn't been opened yet and if it's locked
  (if (not (Variables|Chest|GetIsOpened))
    (if (not (Variables|Chest|GetIsOpening))
      (Variables|Chest|SetIsOpening true)
      ;[1 1 1] Play the open animation
      (bind (_direction _lidalpha) (Timeline|ChestOpenTimeline Play)
        (:Update
          (Transformation|SetRelativeRotation (Variables|Default|GetLidHinge) (Math|Rotator|Lerp(Rotator) "0, 0, 0" (Variables|Chest|GetChestLidOpenAmount) _lidalpha) false false))
        (:Finished
          ;[1 1 1] Finished, set some vars and let everyone know!
          (switch Utilities|FlowControl|Switch|SwitchonETimelineDirection _direction
            (:Forward
              (Variables|Chest|SetIsOpened true)
              (Variables|Chest|SetIsOpening false)
              ;[1 1 1] Spawn the thing
              (if (Variables|Chest|GetSpawnPickupWhenOpened)
                (bind _returnvalue (Game|SpawnActorfromClass "/Game/Blueprints/Ingredients/QuestPickup.QuestPickup_C" (Math|Transform|MakeTransform (Transformation|GetWorldLocation (Variables|Default|GetArrow)) (Transformation|GetActorRotation) "1,1,1.000000") "AdjustIfPossibleButDontSpawnIfColliding" 0 (Variables|Chest|GetPickupType) (Variables|Chest|GetPotionStrength) (Variables|Chest|GetKeyType) (Variables|Chest|GetGoldAmount)))
                (Default|CallOnChestOpened (Variables|Chest|GetPlayerInteracted) _returnvalue)
                (else
                  (Default|CallOnChestOpened (Variables|Chest|GetPlayerInteracted)))))))))))

(event EventPlayerInteract
  ;[1 1 1] Interact or event is called
  ;[1 1 1] Check if locked
  (if (not (Variables|Chest|GetLocked))
    (Variables|Chest|SetPlayerInteracted true)
    ;[1 1 1] Make sure to check if it hasn't been opened yet and if it's locked
    (if (not (Variables|Chest|GetIsOpened))
      (if (not (Variables|Chest|GetIsOpening))
        (Variables|Chest|SetIsOpening true)
        ;[1 1 1] Play the open animation
        (bind (_direction _lidalpha) (Timeline|ChestOpenTimeline Play)
          (:Update
            (Transformation|SetRelativeRotation (Variables|Default|GetLidHinge) (Math|Rotator|Lerp(Rotator) "0, 0, 0" (Variables|Chest|GetChestLidOpenAmount) _lidalpha) false false))
          (:Finished
            ;[1 1 1] Finished, set some vars and let everyone know!
            (switch Utilities|FlowControl|Switch|SwitchonETimelineDirection _direction
              (:Forward
                (Variables|Chest|SetIsOpened true)
                (Variables|Chest|SetIsOpening false)
                ;[1 1 1] Spawn the thing
                (if (Variables|Chest|GetSpawnPickupWhenOpened)
                  (bind _returnvalue (Game|SpawnActorfromClass "/Game/Blueprints/Ingredients/QuestPickup.QuestPickup_C" (Math|Transform|MakeTransform (Transformation|GetWorldLocation (Variables|Default|GetArrow)) (Transformation|GetActorRotation) "1,1,1.000000") "AdjustIfPossibleButDontSpawnIfColliding" 0 (Variables|Chest|GetPickupType) (Variables|Chest|GetPotionStrength) (Variables|Chest|GetKeyType) (Variables|Chest|GetGoldAmount)))
                  (Default|CallOnChestOpened (Variables|Chest|GetPlayerInteracted) _returnvalue)
                  (else
                    (Default|CallOnChestOpened (Variables|Chest|GetPlayerInteracted))))))))))))

(fn ConstructionScript
  (Chest|SetChestMeshes)
  (Chest|SetLidHinge)
  ;[1 1 1] Start with the highlight
  (CallFunction|SetActorHighlightOutline self (Variables|Chest|GetBeginWithHighlightOutline)))

(fn SetLidHinge
  (Transformation|SetRelativeLocation (Variables|Default|GetLidHinge) (Utilities|Select :Index (Variables|Chest|GetChestType) :NewEnumerator0 (Variables|Chest|GetHingeOffsetSmall) :NewEnumerator1 (Variables|Chest|GetHingeOffsetMedium) :NewEnumerator2 (Variables|Chest|GetHingeOffsetLarge) :NewEnumerator3 (Variables|Chest|GetHingeOffsetEpic)) false false)
  (Class|SceneComponent|Attachto (Variables|Default|GetLid) (Variables|Default|GetLidHinge) "None" "KeepWorldPosition" true))

(fn SetChestMeshes
  ;[1 1 1] Set the meshes based off what type of chest it is
  (Components|StaticMesh|SetStaticMesh (Variables|Default|GetBase) (Utilities|Select :Index (Variables|Chest|GetChestType) :NewEnumerator0 "/Game/Props/Chests/Meshes/Chest_Small_Base.Chest_Small_Base" :NewEnumerator1 "/Game/Props/Chests/Meshes/Chest_Medium_Mesh_Base.Chest_Medium_Mesh_Base" :NewEnumerator2 "/Game/Props/Chests/Meshes/Chest_Large_Mesh_Base.Chest_Large_Mesh_Base" :NewEnumerator3 "/Game/Props/Chests/Meshes/Chest_Epic_Mesh_Base.Chest_Epic_Mesh_Base"))
  (Components|StaticMesh|SetStaticMesh (Variables|Default|GetLid) (Utilities|Select :Index (Variables|Chest|GetChestType) :NewEnumerator0 "/Game/Props/Chests/Meshes/Chest_Small_Lid.Chest_Small_Lid" :NewEnumerator1 "/Game/Props/Chests/Meshes/Chest_Medium_Mesh_Lid.Chest_Medium_Mesh_Lid" :NewEnumerator2 "/Game/Props/Chests/Meshes/Chest_Large_Mesh_Lid.Chest_Large_Mesh_Lid" :NewEnumerator3 "/Game/Props/Chests/Meshes/Chest_Epic_Mesh_Lid.Chest_Epic_Mesh_Lid"))
  (Components|StaticMesh|SetStaticMesh (Variables|Default|GetGold) (Utilities|Select :Index (Variables|Chest|GetChestType) :NewEnumerator0 "/Game/Props/Chests/Meshes/Chest_Small_Gold.Chest_Small_Gold" :NewEnumerator1 "/Game/Props/Chests/Meshes/Chest_Medium_Mesh_Gold.Chest_Medium_Mesh_Gold" :NewEnumerator2 "/Game/Props/Chests/Meshes/Chest_Large_Mesh_Gold.Chest_Large_Mesh_Gold" :NewEnumerator3 "/Game/Props/Chests/Meshes/Chest_Epic_Mesh_Gold.Chest_Epic_Mesh_Gold"))
  (Components|StaticMesh|SetStaticMesh (Variables|Default|GetBaseSpiderweb) (Utilities|Select :Index (Variables|Chest|GetChestType) :NewEnumerator0 "/Game/Props/Chests/Meshes/Chest_Small_Spiderweb.Chest_Small_Spiderweb" :NewEnumerator1 "/Game/Props/Chests/Meshes/Chest_Medium_Mesh_Spiderweb.Chest_Medium_Mesh_Spiderweb" :NewEnumerator2 "/Game/Props/Chests/Meshes/Chest_Large_Mesh_BaseSpiderweb.Chest_Large_Mesh_BaseSpiderweb" :NewEnumerator3 "/Game/Props/Chests/Meshes/Chest_Epic_Mesh_BaseSpiderweb.Chest_Epic_Mesh_BaseSpiderweb"))
  (Components|StaticMesh|SetStaticMesh (Variables|Default|GetLidSpiderweb) (Utilities|Select :Index (Variables|Chest|GetChestType) :NewEnumerator0 0 :NewEnumerator1 0 :NewEnumerator2 "/Game/Props/Chests/Meshes/Chest_Large_Mesh_LidSpiderwebs.Chest_Large_Mesh_LidSpiderwebs" :NewEnumerator3 "/Game/Props/Chests/Meshes/Chest_Epic_Mesh_LidSpiderwebs.Chest_Epic_Mesh_LidSpiderwebs"))
  (Components|StaticMesh|SetStaticMesh (Variables|Default|GetInnerShadow) (Utilities|Select :Index (Variables|Chest|GetChestType) :NewEnumerator0 "/Game/Props/Chests/Meshes/Chest_Small_InnerShadow.Chest_Small_InnerShadow" :NewEnumerator1 "/Game/Props/Chests/Meshes/Chest_Medium_Mesh_InnerShadow.Chest_Medium_Mesh_InnerShadow" :NewEnumerator2 "/Game/Props/Chests/Meshes/Chest_Large_Mesh_InnerShadow.Chest_Large_Mesh_InnerShadow" :NewEnumerator3 "/Game/Props/Chests/Meshes/Chest_Epic_Mesh_InnerShadow.Chest_Epic_Mesh_InnerShadow"))
  (Components|StaticMesh|SetStaticMesh (Variables|Default|GetOuterShadow) (Utilities|Select :Index (Variables|Chest|GetChestType) :NewEnumerator0 "/Game/Props/Chests/Meshes/Chest_Small_Outershadow.Chest_Small_Outershadow" :NewEnumerator1 "/Game/Props/Chests/Meshes/Chest_Medium_Mesh_OuterShadow.Chest_Medium_Mesh_OuterShadow" :NewEnumerator2 "/Game/Props/Chests/Meshes/Chest_Large_Mesh_OuterShadow.Chest_Large_Mesh_OuterShadow" :NewEnumerator3 "/Game/Props/Chests/Meshes/Chest_Epic_Mesh_OuterShadow.Chest_Epic_Mesh_OuterShadow"))
  ;[1 1 1] Lock
  (Components|StaticMesh|SetStaticMesh (Variables|Default|GetLock) (Utilities|Select :Index (Variables|Chest|GetChestType) :NewEnumerator0 "/Game/Props/Loot/Meshes/PropLoot_Padlock_Silver.PropLoot_Padlock_Silver" :NewEnumerator1 "/Game/Props/Loot/Meshes/PropLoot_Padlock_Silver.PropLoot_Padlock_Silver" :NewEnumerator2 "/Game/Props/Loot/Meshes/PropLoot_Padlock_Gold.PropLoot_Padlock_Gold" :NewEnumerator3 "/Game/Props/Loot/Meshes/PropLoot_Padlock_Gold.PropLoot_Padlock_Gold"))
  (Transformation|SetRelativeScale3D (Variables|Default|GetLock) (Utilities|Select :Index (Variables|Chest|GetChestType) :NewEnumerator0 "0.500000,0.500000,0.500000" :NewEnumerator1 "0.600000,0.600000,0.600000" :NewEnumerator2 "0.500000,0.500000,0.500000" :NewEnumerator3 "0.800000,0.800000,0.800000"))
  (Transformation|SetRelativeLocation (Variables|Default|GetLock) (Utilities|Select :Index (Variables|Chest|GetChestType) :NewEnumerator0 "0.000000,14.000000,15.000000" :NewEnumerator1 "0.000000,20.000000,10.000000" :NewEnumerator2 "0.000000,20.000000,15.000000" :NewEnumerator3 "0.000000,20.000000,15.000000") false false)
  (Rendering|SetVisibility (Variables|Default|GetLock) (Variables|Chest|GetLocked) false))

(fn SetChestLocked
  (params (Locked :type Boolean :default false))
  (bind _output_get (Variables|Chest|SetLocked Locked))
  (Rendering|SetVisibility (Variables|Default|GetLock) _output_get false))

(fn GetChestIsOpen
  (return (Variables|Chest|GetIsOpened)))

(fn GetChestLocked
  (return (Variables|Chest|GetLocked)))