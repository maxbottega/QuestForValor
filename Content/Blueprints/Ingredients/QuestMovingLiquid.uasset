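; QuestMovingLiquid is a configurable moving liquid surface, offering clear or murky water and bright or dark lava.
; Its Construction Script creates a dynamic material instance from the material matching the selected liquid type.
; It then scales the surface plane in X and Y from user settings and passes speed, scale, displacement, tessellation and opacity values to the material.
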(fn ConstructionScript
  ;[1 1 1] Create the dynamic material instance so that we may modify it at runtime
  (bind _returnvalue (Rendering|Material|CreateDynamicMaterialInstance (Variables|Default|GetLiquidSurface) 0 (Utilities|Select :Index (Variables|MovingLiquid|GetLiquidType) :NewEnumerator0 "/Game/Environment/MovingLiquid/Materials/Environment_MovingLiquid_WaterClear.Environment_MovingLiquid_WaterClear" :NewEnumerator1 "/Game/Environment/MovingLiquid/Materials/Environment_MovingLiquid_WaterMurky.Environment_MovingLiquid_WaterMurky" :NewEnumerator2 "/Game/Environment/MovingLiquid/Materials/Environment_MovingLiquid_Lava01.Environment_MovingLiquid_Lava01" :NewEnumerator3 "/Game/Environment/MovingLiquid/Materials/Environment_MovingLiquid_Lava02.Environment_MovingLiquid_Lava02") :!class /Script/Engine.PrimitiveComponent))
  (Variables|MovingLiquid|SetLiquid%20Material%20Dynamic _returnvalue)
  ;[1 1 1] Set the scale of the plane based off user settings
  (Transformation|SetRelativeScale3D (Variables|Default|GetLiquidSurface) (Math|Vector|MakeVector (Variables|MovingLiquid|GetLiquid%20Scale%20X) (Variables|MovingLiquid|GetLiquid%20Scale%20Y) 1.0))
  ;[1 1 1] Set the properties in the dynamic material insance based off user input
  (Rendering|Material|SetScalarParameterValue (Variables|MovingLiquid|GetLiquid%20Material%20Dynamic) "LiquidSpeed" (Variables|MovingLiquid|GetOverall%20Liqud%20Speed) :!class /Script/Engine.MaterialInstanceDynamic)
  (Rendering|Material|SetScalarParameterValue (Variables|MovingLiquid|GetLiquid%20Material%20Dynamic) "LiquidScale" (Variables|MovingLiquid|GetOverall%20Liquid%20Scale) :!class /Script/Engine.MaterialInstanceDynamic)
  (Rendering|Material|SetScalarParameterValue (Variables|MovingLiquid|GetLiquid%20Material%20Dynamic) "Displacement" (Variables|MovingLiquid|GetDisplacement) :!class /Script/Engine.MaterialInstanceDynamic)
  (Rendering|Material|SetScalarParameterValue (Variables|MovingLiquid|GetLiquid%20Material%20Dynamic) "Tesselation" (Variables|MovingLiquid|GetTesselation%20Factor) :!class /Script/Engine.MaterialInstanceDynamic)
  (Rendering|Material|SetScalarParameterValue (Variables|MovingLiquid|GetLiquid%20Material%20Dynamic) "Opacity" (Variables|MovingLiquid|GetOpacity) :!class /Script/Engine.MaterialInstanceDynamic))