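; Pushable dungeon block that slides a scaled distance away from the player on interaction, with its direction rounded to the block's axes.
; A box trace checks the path, and a hack reverses repeated blocked pushes to free blocks stuck against walls.
; After pushes and on a looping timer, unsupported blocks drop to the traced ground, damaging characters they hit.
; Construction scales distance, trace size and speed, warning on non-uniform scale.
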(event OnComponentBeginOverlap(BlockKillCollision)
  (params (OtherActor :type Actor%20Object%20Reference) (OtherComp :type Primitive%20Component%20Object%20Reference) (OtherBodyIndex :type Integer) (bFromSweep :type Boolean) (SweepResult :type Hit%20Result%20Structure%20%28by%20ref%29))
  ;[1 1 1] When we crushed something
  ;[1 1 1] Only if we're moving
  (if (Variables|PushableBlock|GetBlockIsFalling)
    ;[1 1 1] If we hit a character, then crush them
    (bind _output_get (Variables|PushableBlock|SetHitActor OtherActor))
    (bind _asquest_character (Utilities|Casting|CastToQuestCharacter _output_get))
    (if (== (Variables|/Script/Engine.Character|GetCapsuleComponent _asquest_character) OtherComp)
      (Game|Damage|ApplyDamage (Variables|PushableBlock|GetHitActor) (Variables|PushableBlock|GetCrushingDamage) 0 self "/Script/Engine.DamageType")
      ;[1 1 1] If it's the player, remove collision for camera
      (Utilities|Casting|CastToQuestCharacter_Juno (Variables|PushableBlock|GetHitActor))
      (Collision|SetCollisionResponsetoChannel (Variables|Default|GetMainBlock) "ECC_Camera" "ECR_Ignore"))))

(event Custom|CheckIfFloating
  ;[1 1 1] Every second or so
  ;[1 1 1] Check to see if we should fall
  (if (not (Variables|PushableBlock|GetBlockIsMoving))
    (bind _shouldfall (CallFunction|CheckShouldFall))
    (if _shouldfall
      (Variables|PushableBlock|SetBlockIsMoving true)
      (CallFunction|SetFallData)
      (CallFunction|PlayFallAnimation))))

(event Custom|PlayFallAnimation
  ;[1 1 1] Play the falling timeline
  (Variables|PushableBlock|SetBlockIsFalling true)
  (Components|Timeline|SetPlayRate (Variables|Default|GetFallingTimeline) 2.0)
  (bind _0_1 (Timeline|FallingTimeline PlayFromStart)
    (:Update
      (Transformation|SetActorLocation (+ (Math|Vector|MakeVector 0.0 0.0 (Math|Float|Lerp 0.0 (Variables|PushableBlock|GetFallDistance) _0_1)) (Variables|PushableBlock|GetNewStartPosition)) false false))
    (:Finished
      (Variables|PushableBlock|SetBlockIsFalling false)
      ;[1 1 1] Set the block to finished moving
      (Variables|PushableBlock|SetBlockIsMoving false)
      (Default|CallBlockFinishedMoving self))))

(event Custom|AttemptPushBlock
  (bind _returnvalue (Transformation|GetActorLocation))
  (bind _returnvalue_2 (Game|GetPlayerCharacter 0))
  (bind _returnvalue_3 (Transformation|GetActorRotation))
  (bind _mainblock (Variables|Default|GetMainBlock))
  (bind _returnvalue_4 (Transformation|GetWorldRotation _mainblock))
  (bind _returnvalue_5 (Transformation|GetActorLocation _returnvalue_2))
  (bind _returnvalue_6 (Math|Rotator|FindLookatRotation _returnvalue _returnvalue_5))
  (bind _returnvalue_7 (Math|Rotator|Delta(Rotator) _returnvalue_6 _returnvalue_3))
  (bind _returnvalue_8 (Math|Vector|GetForwardVector _returnvalue_7))
  ;[1 1 1] Events
  ;[1 1 1] Make sure the block isn't moving
  (if (not (Variables|PushableBlock|GetBlockIsMoving))
    ;[1 1 1] Get its new start position
    (Variables|PushableBlock|SetNewStartPosition (Transformation|GetActorLocation))
    ;[1 1 1] Get which direction the push came from
    (Variables|PushableBlock|SetNewForwardVector (Math|Vector|NegateVector (Math|Vector|MakeVector (Math|Conversions|ToFloat(Integer) (Math|Float|Round (.x _returnvalue_8))) (Math|Conversions|ToFloat(Integer) (Math|Float|Round (.y _returnvalue_8))) (Math|Conversions|ToFloat(Integer) (Math|Float|Round (.z _returnvalue_8))))))
    ;[1 1 1] Make sure there's nothing in the way
    (bind _outactors (Actor|GetAllActorsOfClass "/Game/Blueprints/Ingredients/QuestDungeonPressurePlate.QuestDungeonPressurePlate_C"))
    ;[1 1 1] Dont worry about characters or pickups
    (Utilities|Array|AppendArray (Variables|Default|GetActorsToIgnore) _outactors)
    (bind _outactors_2 (Actor|GetAllActorsOfClass "/Game/Blueprints/Ingredients/QuestPickup.QuestPickup_C"))
    (Utilities|Array|AppendArray (Variables|Default|GetActorsToIgnore) _outactors_2)
    (bind _returnvalue_9 (Collision|BoxTraceByChannel (+ (* (.location (Transformation|GetRelativeTransform _mainblock)) (Variables|PushableBlock|GetUniformScale)) (Variables|PushableBlock|GetNewStartPosition)) (+ (+ (* (.location (Transformation|GetRelativeTransform _mainblock)) (Variables|PushableBlock|GetUniformScale)) (Variables|PushableBlock|GetNewStartPosition)) (* (Math|Vector|RotateVector (Variables|PushableBlock|GetNewForwardVector) _returnvalue_4) (Variables|PushableBlock|GetBlockPushingDistance))) (Variables|PushableBlock|GetTraceBoxHalfSize) _returnvalue_4 "TraceTypeQuery1" true (Variables|Default|GetActorsToIgnore) "None"))
    (if (not _returnvalue_9)
      (Variables|PushableBlock|SetLastForwardVector (Variables|PushableBlock|GetNewForwardVector))
      (else
        (|HACK:Preventblocksgettingstuckagainstwalls)))
    ;[1 1 1] Set the block to moving
    (Variables|PushableBlock|SetBlockIsMoving true)
    (Default|CallBlockStartedMoving self)
    ;[1 1 1] Animate the block
    (bind _0_1 (Timeline|BlockPushingTimeline PlayFromStart)
      (:Update
        (Transformation|SetActorLocation (+ (* (Math|Vector|MakeVector (Math|Float|Lerp 0.0 (Variables|PushableBlock|GetBlockPushingDistance) _0_1) (Math|Float|Lerp 0.0 (Variables|PushableBlock|GetBlockPushingDistance) _0_1) 0.0) (Math|Vector|RotateVector (Variables|PushableBlock|GetNewForwardVector) (Transformation|GetWorldRotation (Variables|Default|GetMainBlock)))) (Variables|PushableBlock|GetNewStartPosition)) true false))
      (:Finished
        ;[1 1 1] Check to see if we should fall
        (bind _shouldfall (CallFunction|CheckShouldFall))
        (if _shouldfall
          (CallFunction|SetFallData)
          (CallFunction|PlayFallAnimation)
          (else
            ;[1 1 1] Set the block to finished moving
            (Variables|PushableBlock|SetBlockIsMoving false)
            (Default|CallBlockFinishedMoving self)))))))

(event EventBeginPlay
  ;[1 1 1] Set a retriggering call to see if the block is floating
  (Utilities|Time|SetTimerbyFunctionName 0 "CheckIfFloating" 1.5 true))

(event EventPlayerInteract
  (bind _returnvalue (Transformation|GetActorLocation))
  (bind _returnvalue_2 (Game|GetPlayerCharacter 0))
  (bind _returnvalue_3 (Transformation|GetActorRotation))
  (bind _mainblock (Variables|Default|GetMainBlock))
  (bind _returnvalue_4 (Transformation|GetWorldRotation _mainblock))
  (bind _returnvalue_5 (Transformation|GetActorLocation _returnvalue_2))
  (bind _returnvalue_6 (Math|Rotator|FindLookatRotation _returnvalue _returnvalue_5))
  (bind _returnvalue_7 (Math|Rotator|Delta(Rotator) _returnvalue_6 _returnvalue_3))
  (bind _returnvalue_8 (Math|Vector|GetForwardVector _returnvalue_7))
  ;[1 1 1] Events
  ;[1 1 1] Make sure the block isn't moving
  (if (not (Variables|PushableBlock|GetBlockIsMoving))
    ;[1 1 1] Get its new start position
    (Variables|PushableBlock|SetNewStartPosition (Transformation|GetActorLocation))
    ;[1 1 1] Get which direction the push came from
    (Variables|PushableBlock|SetNewForwardVector (Math|Vector|NegateVector (Math|Vector|MakeVector (Math|Conversions|ToFloat(Integer) (Math|Float|Round (.x _returnvalue_8))) (Math|Conversions|ToFloat(Integer) (Math|Float|Round (.y _returnvalue_8))) (Math|Conversions|ToFloat(Integer) (Math|Float|Round (.z _returnvalue_8))))))
    ;[1 1 1] Make sure there's nothing in the way
    (bind _outactors (Actor|GetAllActorsOfClass "/Game/Blueprints/Ingredients/QuestDungeonPressurePlate.QuestDungeonPressurePlate_C"))
    ;[1 1 1] Dont worry about characters or pickups
    (Utilities|Array|AppendArray (Variables|Default|GetActorsToIgnore) _outactors)
    (bind _outactors_2 (Actor|GetAllActorsOfClass "/Game/Blueprints/Ingredients/QuestPickup.QuestPickup_C"))
    (Utilities|Array|AppendArray (Variables|Default|GetActorsToIgnore) _outactors_2)
    (bind _returnvalue_9 (Collision|BoxTraceByChannel (+ (* (.location (Transformation|GetRelativeTransform _mainblock)) (Variables|PushableBlock|GetUniformScale)) (Variables|PushableBlock|GetNewStartPosition)) (+ (+ (* (.location (Transformation|GetRelativeTransform _mainblock)) (Variables|PushableBlock|GetUniformScale)) (Variables|PushableBlock|GetNewStartPosition)) (* (Math|Vector|RotateVector (Variables|PushableBlock|GetNewForwardVector) _returnvalue_4) (Variables|PushableBlock|GetBlockPushingDistance))) (Variables|PushableBlock|GetTraceBoxHalfSize) _returnvalue_4 "TraceTypeQuery1" true (Variables|Default|GetActorsToIgnore) "None"))
    (if (not _returnvalue_9)
      (Variables|PushableBlock|SetLastForwardVector (Variables|PushableBlock|GetNewForwardVector))
      (else
        (|HACK:Preventblocksgettingstuckagainstwalls)))
    ;[1 1 1] Set the block to moving
    (Variables|PushableBlock|SetBlockIsMoving true)
    (Default|CallBlockStartedMoving self)
    ;[1 1 1] Animate the block
    (bind _0_1 (Timeline|BlockPushingTimeline PlayFromStart)
      (:Update
        (Transformation|SetActorLocation (+ (* (Math|Vector|MakeVector (Math|Float|Lerp 0.0 (Variables|PushableBlock|GetBlockPushingDistance) _0_1) (Math|Float|Lerp 0.0 (Variables|PushableBlock|GetBlockPushingDistance) _0_1) 0.0) (Math|Vector|RotateVector (Variables|PushableBlock|GetNewForwardVector) (Transformation|GetWorldRotation (Variables|Default|GetMainBlock)))) (Variables|PushableBlock|GetNewStartPosition)) true false))
      (:Finished
        ;[1 1 1] Check to see if we should fall
        (bind _shouldfall (CallFunction|CheckShouldFall))
        (if _shouldfall
          (CallFunction|SetFallData)
          (CallFunction|PlayFallAnimation)
          (else
            ;[1 1 1] Set the block to finished moving
            (Variables|PushableBlock|SetBlockIsMoving false)
            (Default|CallBlockFinishedMoving self)))))))

(fn ConstructionScript
  (CallFunction|SettoNewScale)
  ;[1 1 1] Set the play rate acording to variables
  (Components|Timeline|SetPlayRate (Variables|Default|GetBlockPushingTimeline) (Variables|PushableBlock|GetBlockPushingPlayRate))
  ;[1 1 1] Start with the highlight
  (CallFunction|SetActorHighlightOutline self (Variables|PushableBlock|GetBeginWithHighlightOutline)))

(fn CheckShouldFall
  (bind _returnvalue (Transformation|GetActorLocation))
  (bind _uniformscale (Variables|PushableBlock|GetUniformScale))
  (bind _mainblock (Variables|Default|GetMainBlock))
  (bind _returnvalue_2 (Transformation|GetRelativeTransform _mainblock))
  (bind _returnvalue_3 (* (.location _returnvalue_2) _uniformscale))
  (bind _returnvalue_4 (+ _returnvalue_3 _returnvalue))
  ;[1 1 1] Check to see if we need to fall
  (bind _outactors (Actor|GetAllActorsOfClass "/Game/Blueprints/Ingredients/QuestDungeonPressurePlate.QuestDungeonPressurePlate_C"))
  (bind _returnvalue_5 (Collision|BoxTraceByChannel _returnvalue_4 (+ _returnvalue_4 (* "0, 0,-1.000000" (Variables|PushableBlock|GetBlockPushingDistance))) (Variables|PushableBlock|GetTraceBoxHalfSize) "0, 0, 0" "TraceTypeQuery1" true _outactors "None"))
  ;[1 1 1] Return
  (return (not _returnvalue_5)))

(fn SetFallData
  (bind _returnvalue (Transformation|GetActorLocation))
  ;[1 1 1] We need to fall! Get some important vars
  (bind _outhit (Collision|LineTraceByChannel _returnvalue (+ _returnvalue (* "0, 0,-1.000000" 1e+04)) "TraceTypeQuery1" false 0 "None"))
  (Variables|PushableBlock|SetFallLocation (.Location (Collision|BreakHitResult _outhit)))
  (Variables|PushableBlock|SetNewStartPosition (Transformation|GetActorLocation))
  (Variables|PushableBlock|SetFallDistance (- (.z (Variables|PushableBlock|GetFallLocation)) (.z (Variables|PushableBlock|GetNewStartPosition))))
  (return))

(fn SettoNewScale
  (bind _returnvalue (Transformation|GetActorScale3D))
  ;[1 1 1] Set tyhe new scale
  (bind _output_get (LocalVariables|SetNewUniformScaleLocal (.x _returnvalue)))
  (Variables|PushableBlock|SetUniformScale _output_get)
  (if (Math|Boolean|ANDBoolean (== (.x _returnvalue) (.y _returnvalue)) (== (.x _returnvalue) (.z _returnvalue)) (== (.y _returnvalue) (.z _returnvalue)))
    (Variables|PushableBlock|SetBlockPushingDistance (* (Variables|PushableBlock|GetBlockPushingDistance) (LocalVariables|GetNewUniformScaleLocal)))
    (Variables|PushableBlock|SetTraceBoxHalfSize (* (Variables|PushableBlock|GetTraceBoxHalfSize) (LocalVariables|GetNewUniformScaleLocal)))
    (Variables|PushableBlock|SetBlockPushingPlayRate (/ (Variables|PushableBlock|GetBlockPushingPlayRate) (LocalVariables|GetNewUniformScaleLocal)))
    (else
      (Development|PrintString "WARNING: The Pushable Block MUST have a uniform X, Y, Z scale!" true true "(R=1.000000,G=0.040325,B=0.000000,A=1.000000)"))))