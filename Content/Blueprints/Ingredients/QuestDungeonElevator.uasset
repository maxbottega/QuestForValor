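; Quest dungeon elevator that travels between its placed position and an editable end transform, triggered by player interaction or script calls.
; A timeline lerps location and rotation with added sway, then unlocks and broadcasts direction and whether the player triggered it.
; Player interaction respects and sets the lock, while CallElevator skips it; both reverse the last finished direction.
; The construction script caches the start, sets speed, optional back end, end preview mesh and highlight.
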(event Custom|PlayElevatorMovement
  (bind _startrotation (Variables|Elevator|GetStartRotation))
  ;[1 1 1] Events
  (Variables|Elevator|SetPlayerInteracted false)
  ;[1 1 1] Play the timeline animation
  (bind (_direction _0_1 _swaying) (Timeline|ElevatorMovementTimeline Play)
    (:Update
      (Transformation|SetWorldLocationAndRotation (Variables|Default|GetScene) (Math|Vector|Lerp(Vector) (Variables|Elevator|GetStartPosition) (+ (Variables|Elevator|GetStartPosition) (Math|Vector|RotateVector (.location (Variables|Elevator|GetEndTransform)) (Variables|Elevator|GetStartRotation))) _0_1) (Math|Rotator|CombineRotators (Math|Rotator|MakeRotator (.Z (Math|Vector|BreakVector _swaying)) (.X (Math|Vector|BreakVector _swaying)) (.Y (Math|Vector|BreakVector _swaying))) (Math|Rotator|Lerp(Rotator) _startrotation (Math|Rotator|CombineRotators _startrotation (.rotation (Variables|Elevator|GetEndTransform))) _0_1 true)) false false))
    (:Finished
      ;[1 1 1] Set states and let everyone know we moved
      (Variables|Elevator|SetLocked false)
      (bind _output_get (Variables|Elevator|SetElevatorLastDirection _direction))
      (Default|CallOnElevatorFinishedMoving _output_get (Variables|Elevator|GetPlayerInteracted)))))

(event Custom|ReverseElevatorMovement
  (bind _startrotation (Variables|Elevator|GetStartRotation))
  ;[1 1 1] Events
  (Variables|Elevator|SetPlayerInteracted false)
  ;[1 1 1] Play the timeline animation
  (bind (_direction _0_1 _swaying) (Timeline|ElevatorMovementTimeline Reverse)
    (:Update
      (Transformation|SetWorldLocationAndRotation (Variables|Default|GetScene) (Math|Vector|Lerp(Vector) (Variables|Elevator|GetStartPosition) (+ (Variables|Elevator|GetStartPosition) (Math|Vector|RotateVector (.location (Variables|Elevator|GetEndTransform)) (Variables|Elevator|GetStartRotation))) _0_1) (Math|Rotator|CombineRotators (Math|Rotator|MakeRotator (.Z (Math|Vector|BreakVector _swaying)) (.X (Math|Vector|BreakVector _swaying)) (.Y (Math|Vector|BreakVector _swaying))) (Math|Rotator|Lerp(Rotator) _startrotation (Math|Rotator|CombineRotators _startrotation (.rotation (Variables|Elevator|GetEndTransform))) _0_1 true)) false false))
    (:Finished
      ;[1 1 1] Set states and let everyone know we moved
      (Variables|Elevator|SetLocked false)
      (bind _output_get (Variables|Elevator|SetElevatorLastDirection _direction))
      (Default|CallOnElevatorFinishedMoving _output_get (Variables|Elevator|GetPlayerInteracted)))))

(event Custom|CallElevator
  (bind _startrotation (Variables|Elevator|GetStartRotation))
  ;[1 1 1] Player or script calls elevator
  ;[1 1 1] Make sure the elevator is not locked
  (Variables|Elevator|SetPlayerInteracted false)
  ;[1 1 1] Check which direction to play
  (switch Utilities|FlowControl|Switch|SwitchonETimelineDirection (Variables|Elevator|GetElevatorLastDirection)
    (:Forward
      ;[1 1 1] Play the timeline animation
      (bind (_direction _0_1 _swaying) (Timeline|ElevatorMovementTimeline Reverse)
        (:Update
          (Transformation|SetWorldLocationAndRotation (Variables|Default|GetScene) (Math|Vector|Lerp(Vector) (Variables|Elevator|GetStartPosition) (+ (Variables|Elevator|GetStartPosition) (Math|Vector|RotateVector (.location (Variables|Elevator|GetEndTransform)) (Variables|Elevator|GetStartRotation))) _0_1) (Math|Rotator|CombineRotators (Math|Rotator|MakeRotator (.Z (Math|Vector|BreakVector _swaying)) (.X (Math|Vector|BreakVector _swaying)) (.Y (Math|Vector|BreakVector _swaying))) (Math|Rotator|Lerp(Rotator) _startrotation (Math|Rotator|CombineRotators _startrotation (.rotation (Variables|Elevator|GetEndTransform))) _0_1 true)) false false))
        (:Finished
          ;[1 1 1] Set states and let everyone know we moved
          (Variables|Elevator|SetLocked false)
          (bind _output_get (Variables|Elevator|SetElevatorLastDirection _direction))
          (Default|CallOnElevatorFinishedMoving _output_get (Variables|Elevator|GetPlayerInteracted)))))
    (:Backward
      (Timeline|ElevatorMovementTimeline Play))))

(event EventPlayerInteract
  (bind _startrotation (Variables|Elevator|GetStartRotation))
  ;[1 1 1] Player or script calls elevator
  ;[1 1 1] Make sure the elevator is not locked
  (if (not (Variables|Elevator|GetLocked))
    (Variables|Elevator|SetLocked true)
    (Variables|Elevator|SetPlayerInteracted true)
    ;[1 1 1] Check which direction to play
    (switch Utilities|FlowControl|Switch|SwitchonETimelineDirection (Variables|Elevator|GetElevatorLastDirection)
      (:Forward
        ;[1 1 1] Play the timeline animation
        (bind (_direction _0_1 _swaying) (Timeline|ElevatorMovementTimeline Reverse)
          (:Update
            (Transformation|SetWorldLocationAndRotation (Variables|Default|GetScene) (Math|Vector|Lerp(Vector) (Variables|Elevator|GetStartPosition) (+ (Variables|Elevator|GetStartPosition) (Math|Vector|RotateVector (.location (Variables|Elevator|GetEndTransform)) (Variables|Elevator|GetStartRotation))) _0_1) (Math|Rotator|CombineRotators (Math|Rotator|MakeRotator (.Z (Math|Vector|BreakVector _swaying)) (.X (Math|Vector|BreakVector _swaying)) (.Y (Math|Vector|BreakVector _swaying))) (Math|Rotator|Lerp(Rotator) _startrotation (Math|Rotator|CombineRotators _startrotation (.rotation (Variables|Elevator|GetEndTransform))) _0_1 true)) false false))
          (:Finished
            ;[1 1 1] Set states and let everyone know we moved
            (Variables|Elevator|SetLocked false)
            (bind _output_get (Variables|Elevator|SetElevatorLastDirection _direction))
            (Default|CallOnElevatorFinishedMoving _output_get (Variables|Elevator|GetPlayerInteracted)))))
      (:Backward
        (Timeline|ElevatorMovementTimeline Play)))))

(fn ConstructionScript
  (bind _endtransform (Variables|Elevator|GetEndTransform))
  (bind (_location _rotation) (Math|Transform|BreakTransform _endtransform))
  ;[1 1 1] Get and save the initial start position
  (Variables|Elevator|SetStartPosition (Transformation|GetWorldLocation (Variables|Default|GetScene)))
  ;[1 1 1] Get the intial rotation
  (Variables|Elevator|SetStartRotation (Transformation|GetWorldRotation (Variables|Default|GetScene)))
  ;[1 1 1] Elevator play rate
  (Components|Timeline|SetPlayRate (Variables|Default|GetElevatorMovementTimeline) (/ 1.0 (Variables|Elevator|GetElevatorMovementSpeed)))
  ;[1 1 1] Remove the back end if we don't want it
  (if (not (Variables|Elevator|GetHasBackEnd))
    (Components|DestroyComponent (Variables|Default|GetStaticMesh14))
    (Components|DestroyComponent (Variables|Default|GetWallCollisionBack)))
  ;[1 1 1] Set the preview mesh's location and it's visibility
  (Transformation|SetRelativeLocationAndRotation (Variables|Default|GetPreviewMesh) _location _rotation false false)
  (Rendering|SetVisibility (Variables|Default|GetPreviewMesh) (not (Variables|Elevator|GetHidePreviewMesh)) true)
  ;[1 1 1] Start with the highlight
  (CallFunction|SetActorHighlightOutline self (Variables|Elevator|GetBeginWithHighlightOutline)))

(fn SetElevatorLocked
  (params (Locked :type Boolean :default false))
  (Variables|Elevator|SetLocked Locked))

(fn GetElevatorLocked
  (return (Variables|Elevator|GetLocked)))