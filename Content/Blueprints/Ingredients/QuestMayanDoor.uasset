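; Mayan temple double door in wood or stone, with an optional archway, that the player or other logic can open, close or toggle.
; One timeline rotates both hinges, swinging by the player's side when interacted with, and plays in reverse to close.
; Locked doors shake on player interaction and show lock meshes while shut and still; open and close calls bypass the lock.
; Completed moves report the door and whether the player triggered them.
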(event Custom|OpenDoor
  ;[1 1 1] Open/close the door only if it's unlocked
  (Variables|Door|SetPlayerInteracted false)
  ;[1 1 1] Comment
  (Variables|Door|SetDoorMoving true)
  (Door|SetDoorLocksVisible (Door|GetShouldLocksbeVisible))
  ;[1 1 1] Animation timeline: Rotate the doors
  (bind (_direction _0_1) (Timeline|OpenDoorTimeline Play)
    (:Update
      (Transformation|SetRelativeRotation (Variables|Default|GetDoorRightHinge) (Math|Rotator|MakeRotator 0.0 0.0 (Math|Float|Lerp 0.0 (* (Variables|Door|GetDoorOpenAngle) (select (Variables|Door|GetDoorOpenForward) 1.0 -1.0)) _0_1)) false false)
      (Transformation|SetRelativeRotation (Variables|Default|GetDoorLeftHinge) (Math|Rotator|MakeRotator 0.0 0.0 (Math|Float|Lerp 0.0 (* (Variables|Door|GetDoorOpenAngle) (select (Variables|Door|GetDoorOpenForward) -1.0 1.0)) _0_1)) false false))
    (:Finished
      (Variables|Door|SetDoorMoving false)
      ;[1 1 1] Set door open state
      (switch Utilities|FlowControl|Switch|SwitchonETimelineDirection _direction
        (:Forward
          (Variables|Door|SetDoorIsOpen true)
          (Door|SetDoorLocksVisible false)
          ;[1 1 1] Let the world know we opened/closed
          (Default|CallDoorOpened self (Variables|Door|GetPlayerInteracted)))
        (:Backward
          (Variables|Door|SetDoorIsOpen false)
          (Door|SetDoorLocksVisible (Door|GetShouldLocksbeVisible))
          (Default|CallDoorClosed self (Variables|Door|GetPlayerInteracted)))))))

(event Custom|CloseDoor
  ;[1 1 1] Open/close the door only if it's unlocked
  (Variables|Door|SetPlayerInteracted false)
  ;[1 1 1] Comment
  (Variables|Door|SetDoorMoving true)
  (Door|SetDoorLocksVisible (Door|GetShouldLocksbeVisible))
  ;[1 1 1] Animation timeline: Rotate the doors
  (bind (_direction _0_1) (Timeline|OpenDoorTimeline Reverse)
    (:Update
      (Transformation|SetRelativeRotation (Variables|Default|GetDoorRightHinge) (Math|Rotator|MakeRotator 0.0 0.0 (Math|Float|Lerp 0.0 (* (Variables|Door|GetDoorOpenAngle) (select (Variables|Door|GetDoorOpenForward) 1.0 -1.0)) _0_1)) false false)
      (Transformation|SetRelativeRotation (Variables|Default|GetDoorLeftHinge) (Math|Rotator|MakeRotator 0.0 0.0 (Math|Float|Lerp 0.0 (* (Variables|Door|GetDoorOpenAngle) (select (Variables|Door|GetDoorOpenForward) -1.0 1.0)) _0_1)) false false))
    (:Finished
      (Variables|Door|SetDoorMoving false)
      ;[1 1 1] Set door open state
      (switch Utilities|FlowControl|Switch|SwitchonETimelineDirection _direction
        (:Forward
          (Variables|Door|SetDoorIsOpen true)
          (Door|SetDoorLocksVisible false)
          ;[1 1 1] Let the world know we opened/closed
          (Default|CallDoorOpened self (Variables|Door|GetPlayerInteracted)))
        (:Backward
          (Variables|Door|SetDoorIsOpen false)
          (Door|SetDoorLocksVisible (Door|GetShouldLocksbeVisible))
          (Default|CallDoorClosed self (Variables|Door|GetPlayerInteracted)))))))

(event Custom|ToggleDoorOpen
  ;[1 1 1] Open/close the door only if it's unlocked
  (Variables|Door|SetPlayerInteracted false)
  (if (not (Variables|Door|GetDoorIsOpen))
    ;[1 1 1] Comment
    (Variables|Door|SetDoorMoving true)
    (Door|SetDoorLocksVisible (Door|GetShouldLocksbeVisible))
    ;[1 1 1] Animation timeline: Rotate the doors
    (bind (_direction _0_1) (Timeline|OpenDoorTimeline Play)
      (:Update
        (Transformation|SetRelativeRotation (Variables|Default|GetDoorRightHinge) (Math|Rotator|MakeRotator 0.0 0.0 (Math|Float|Lerp 0.0 (* (Variables|Door|GetDoorOpenAngle) (select (Variables|Door|GetDoorOpenForward) 1.0 -1.0)) _0_1)) false false)
        (Transformation|SetRelativeRotation (Variables|Default|GetDoorLeftHinge) (Math|Rotator|MakeRotator 0.0 0.0 (Math|Float|Lerp 0.0 (* (Variables|Door|GetDoorOpenAngle) (select (Variables|Door|GetDoorOpenForward) -1.0 1.0)) _0_1)) false false))
      (:Finished
        (Variables|Door|SetDoorMoving false)
        ;[1 1 1] Set door open state
        (switch Utilities|FlowControl|Switch|SwitchonETimelineDirection _direction
          (:Forward
            (Variables|Door|SetDoorIsOpen true)
            (Door|SetDoorLocksVisible false)
            ;[1 1 1] Let the world know we opened/closed
            (Default|CallDoorOpened self (Variables|Door|GetPlayerInteracted)))
          (:Backward
            (Variables|Door|SetDoorIsOpen false)
            (Door|SetDoorLocksVisible (Door|GetShouldLocksbeVisible))
            (Default|CallDoorClosed self (Variables|Door|GetPlayerInteracted))))))
    (else
      (Variables|Door|SetDoorMoving true)
      (Door|SetDoorLocksVisible (Door|GetShouldLocksbeVisible))
      (Timeline|OpenDoorTimeline Reverse))))

(event EventBeginPlay
  ;[1 1 1] Check if the door is open by default
  (if (Variables|Door|GetOpenByDefault)
    (Components|Timeline|SetPlaybackPosition (Variables|Default|GetOpenDoorTimeline) 1.0 true true)))

(event EventPlayerInteract
  ;[1 1 1] Player interaction
  (if (not (Variables|Door|GetLocked))
    (Variables|Door|SetPlayerInteracted true)
    ;[1 1 1] Comment
    (if (and (not (Variables|Door|GetDoorMoving)) (not (Variables|Door|GetDoorIsOpen)))
      (Variables|Door|SetDoorOpenForward (> (Math|Vector|DotProduct (Class|KismetMathLibrary|GetDirectionVector (Transformation|GetActorLocation) (Transformation|GetActorLocation (Game|GetPlayerCharacter 0))) (Transformation|GetActorRightVector)) 0.0)))
    ;[1 1 1] Open/close the door only if it's unlocked
    (if (not (Variables|Door|GetDoorIsOpen))
      ;[1 1 1] Comment
      (Variables|Door|SetDoorMoving true)
      (Door|SetDoorLocksVisible (Door|GetShouldLocksbeVisible))
      ;[1 1 1] Animation timeline: Rotate the doors
      (bind (_direction _0_1) (Timeline|OpenDoorTimeline Play)
        (:Update
          (Transformation|SetRelativeRotation (Variables|Default|GetDoorRightHinge) (Math|Rotator|MakeRotator 0.0 0.0 (Math|Float|Lerp 0.0 (* (Variables|Door|GetDoorOpenAngle) (select (Variables|Door|GetDoorOpenForward) 1.0 -1.0)) _0_1)) false false)
          (Transformation|SetRelativeRotation (Variables|Default|GetDoorLeftHinge) (Math|Rotator|MakeRotator 0.0 0.0 (Math|Float|Lerp 0.0 (* (Variables|Door|GetDoorOpenAngle) (select (Variables|Door|GetDoorOpenForward) -1.0 1.0)) _0_1)) false false))
        (:Finished
          (Variables|Door|SetDoorMoving false)
          ;[1 1 1] Set door open state
          (switch Utilities|FlowControl|Switch|SwitchonETimelineDirection _direction
            (:Forward
              (Variables|Door|SetDoorIsOpen true)
              (Door|SetDoorLocksVisible false)
              ;[1 1 1] Let the world know we opened/closed
              (Default|CallDoorOpened self (Variables|Door|GetPlayerInteracted)))
            (:Backward
              (Variables|Door|SetDoorIsOpen false)
              (Door|SetDoorLocksVisible (Door|GetShouldLocksbeVisible))
              (Default|CallDoorClosed self (Variables|Door|GetPlayerInteracted))))))
      (else
        (Variables|Door|SetDoorMoving true)
        (Door|SetDoorLocksVisible (Door|GetShouldLocksbeVisible))
        (Timeline|OpenDoorTimeline Reverse)))
    (else
      ;[1 1 1] Animation timeline: Shake the doors if they are locked
      (if (not (Variables|Door|GetDoorIsOpen))
        (bind _0_1_2 (Timeline|DoorLockedShakeAnimation PlayFromStart)
          (:Update
            (Transformation|SetRelativeRotation (Variables|Default|GetDoorRightHinge) (Math|Rotator|MakeRotator 0.0 0.0 (Math|Float|Lerp 0.0 (Variables|Door|GetDoorLockedShakeAngle) _0_1_2)) false false)
            (Transformation|SetRelativeRotation (Variables|Default|GetDoorLeftHinge) (Math|Rotator|MakeRotator 0.0 0.0 (Math|Float|Lerp 0.0 (* (Variables|Door|GetDoorLockedShakeAngle) -1.0) _0_1_2)) false false)))))))

(fn ConstructionScript
  ;[1 1 1] Set how fast the door will open
  (Components|Timeline|SetPlayRate (Variables|Default|GetOpenDoorTimeline) (Variables|Door|GetDoorOpenPlayRate))
  ;[1 1 1] Set the door type
  (Door|SetDoorType (Variables|Door|GetDoorType))
  ;[1 1 1] Add the archway mesh
  (if (Variables|Door|GetIncludeArchwayMesh)
    (Components|StaticMesh|SetStaticMesh (Variables|Default|GetArchway) "/Game/Environment/MayanTemple/Meshes/MayanTemple_Arch.MayanTemple_Arch")
    ;[1 1 1] If the door is open or not
    (Variables|Door|SetDoorIsOpen (Variables|Door|GetOpenByDefault))
    ;[1 1 1] Start with the highlight
    (CallFunction|SetActorHighlightOutline self (Variables|Door|GetBeginWithHighlightOutline))
    ;[1 1 1] Comment
    (Door|SetDoorLocksVisible (and (Door|GetShouldLocksbeVisible) (not (Variables|Door|GetOpenByDefault))))))

(fn SetDoorType
  (params (NewDoorType :type Enum_MayanDoorTypes%20Enum :default "NewEnumerator0"))
  ;[1 1 1] Init vars
  (LocalVariables|SetNewDoorTypeLocal NewDoorType)
  ;[1 1 1] Set the meshes based off the door type
  (Components|StaticMesh|SetStaticMesh (Variables|Default|GetDoorFrame) (Utilities|Select :Index (LocalVariables|GetNewDoorTypeLocal) :NewEnumerator0 "/Game/Environment/MayanTemple/Meshes/MayanTemple_Door_Wood_Frame.MayanTemple_Door_Wood_Frame" :NewEnumerator1 "/Game/Environment/MayanTemple/Meshes/MayanTemple_Door_Stone_Frame.MayanTemple_Door_Stone_Frame"))
  (Components|StaticMesh|SetStaticMesh (Variables|Default|GetDoorLeft) (Utilities|Select :Index (LocalVariables|GetNewDoorTypeLocal) :NewEnumerator0 "/Game/Environment/MayanTemple/Meshes/MayanTemple_Door_Wood_Left.MayanTemple_Door_Wood_Left" :NewEnumerator1 "/Game/Environment/MayanTemple/Meshes/MayanTemple_Door_Stone_Left.MayanTemple_Door_Stone_Left"))
  (Components|StaticMesh|SetStaticMesh (Variables|Default|GetDoorRight) (Utilities|Select :Index (LocalVariables|GetNewDoorTypeLocal) :NewEnumerator0 "/Game/Environment/MayanTemple/Meshes/MayanTemple_Door_Wood_Right.MayanTemple_Door_Wood_Right" :NewEnumerator1 "/Game/Environment/MayanTemple/Meshes/MayanTemple_Door_Stone_Right.MayanTemple_Door_Stone_Right"))
  ;[1 1 1] Return
  (return))

(fn SetDoorLocked
  (params (Locked :type Boolean :default false))
  (Variables|Door|SetLocked Locked)
  (Door|SetDoorLocksVisible (Door|GetShouldLocksbeVisible)))

(fn GetDoorIsOpen
  (return (Variables|Door|GetDoorIsOpen)))

(fn SetDoorLocksVisible
  (params (bNewVisibility :type Boolean))
  (Rendering|SetVisibility (Variables|Default|GetLock01) bNewVisibility false))

(fn GetShouldLocksbeVisible
  (return (Math|Boolean|ANDBoolean (Variables|Door|GetLocked) (not (Variables|Door|GetDoorIsOpen)) (not (Variables|Door|GetDoorMoving)))))

(fn GetDoorLocked
  (return (Variables|Door|GetLocked)))