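; Quest trigger actor that fires OnLookedAt and OnUnlookedAt events as the player (Juno) gains or loses sight of it.
; While Juno is inside the resizable sphere, a looping timer runs a camera-to-actor multi line trace and a world-to-screen projection check.
; Paired DoOnce nodes reset each other so events fire only on state changes.
; Leaving the sphere stops the timer and re-arms the looked-at event.
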(event OnComponentBeginOverlap(PlayerEnterArea)
  (params (OtherActor :type Actor%20Object%20Reference) (OtherComp :type Primitive%20Component%20Object%20Reference) (OtherBodyIndex :type Integer) (bFromSweep :type Boolean) (SweepResult :type Hit%20Result%20Structure%20%28by%20ref%29))
  ;[1 1 1] Comment
  (Utilities|Casting|CastToQuestCharacter_Juno OtherActor)
  (bind _returnvalue (Utilities|Time|SetTimerbyEvent (delegate Custom|CheckLineOfSight) (Variables|LookAtTrigger|GetCheckTickTime) true)))

(event OnComponentEndOverlap(PlayerEnterArea)
  (params (OtherActor :type Actor%20Object%20Reference) (OtherComp :type Primitive%20Component%20Object%20Reference) (OtherBodyIndex :type Integer))
  ;[1 1 1] Comment
  (Utilities|Casting|CastToQuestCharacter_Juno OtherActor)
  (Class|KismetSystemLibrary|ClearTimerHandle (stale OnComponentBeginOverlap(PlayerEnterArea) _returnvalue))
  ;[1 1 1] Comment
  (Utilities|FlowControl|DoOnce false) ; enters at Reset
)

(event Custom|CheckLineOfSight
  ;[1 1 1] Comment
  (bind _outhits (Class|KismetSystemLibrary|LineTraceMultiNEW (Camera|GetCameraLocation (Game|GetPlayerCameraManager 0)) (Transformation|GetActorLocation self) "TraceTypeQuery2" true (Utilities|Array|MakeArray (Game|GetPlayerCharacter 0)) "None" false))
  ;[1 1 1] Comment
  (Variables|LookAtTrigger|SetCurrentlyLookedAt false)
  (bind _array_element (Utilities|Array|ForEachLoopwithBreak _outhits)
    (:LoopBody
      (if (== (.HitActor (Collision|BreakHitResult _array_element)) self)
        (Variables|LookAtTrigger|SetCurrentlyLookedAt true)))
    (:Completed
      ;[1 1 1] Comment
      (if (and (Variables|LookAtTrigger|GetCurrentlyLookedAt) (.ReturnValue (Class|GameplayStatics|ProjectWorldtoScreen (Game|GetPlayerController 0) (Transformation|GetWorldLocation (Variables|Default|GetLookAtTrigger)))))
        (Utilities|FlowControl|DoOnce false :!label _label
          (:Completed
            (Default|CallOnLookedat self)
            (goto _label_2 Reset)))
        (else
          (Utilities|FlowControl|DoOnce false :!label _label_2
            (:Completed
              (Default|CallOnUnlookedat self)
              (goto _label Reset))))))))

(fn ConstructionScript
  ;[1 1 1] Set size
  (Components|Sphere|SetSphereRadius (Variables|Default|GetPlayerEnterArea) (Variables|LookAtTrigger|GetSize) true)
  ;[1 1 1] Debug: Set visibility
  (Development|SetHiddeninGame (Variables|Default|GetPlayerEnterArea) (not (Variables|LookAtTrigger|GetDebugDrawInGame)) false))