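; QuestMarker is an actor Blueprint for a quest marker that can be switched on or off and carries a marker type.
; SetMarkerActive stores the Active flag and passes the marker to the Game Instance through SetMarkerMessage or ClearMarkerMessage, and BeginPlay applies the initial state this way.
; A simple setter and getter expose MarkerType, with no display logic in its graphs.
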(event EventBeginPlay
  (Marker|SetMarkerActive (Variables|Marker|GetActive)))

(event EventActorBeginOverlap
  (params (OtherActor :type Actor%20Object%20Reference)))

(event EventTick
  (params (DeltaSeconds :type Float%20%28single-precision%29)))

(fn ConstructionScript)

(fn SetMarkerActive
  (params (Active :type Boolean))
  (bind _output_get (Variables|Marker|SetActive Active))
  (if _output_get
    (Class|QuestMarkerInterface|SetMarker(Message) (Game|GetGameInstance) self)
    (else
      (Class|QuestMarkerInterface|ClearMarker(Message) (Game|GetGameInstance) self))))

(fn SetMarkerType
  (params (MarkerType :type Enum_MarkerType%20Enum :default "NewEnumerator0"))
  (Variables|Marker|SetMarkerType MarkerType))

(fn GetMarkerType
  (return (Variables|Marker|GetMarkerType)))