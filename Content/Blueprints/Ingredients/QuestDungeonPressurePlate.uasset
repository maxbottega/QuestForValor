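; Quest dungeon pressure plate that sinks when a quest character's capsule or a pushable block rests on it, optionally accepting only blocks.
; It counts valid overlaps, including actors present at BeginPlay, and plays a movement timeline for the first arrival, reversing when the last leaves unless set to one-time activation.
; When the timeline finishes, it updates its down state and broadcasts activated or deactivated events.
; Construction sets animation speed and optional starting highlight outline.
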(event OnComponentBeginOverlap(PressurePlateCollision)
  (params (OverlappedComponent :type Primitive%20Component%20Object%20Reference) (OtherActor :type Actor%20Object%20Reference) (OtherComp :type Primitive%20Component%20Object%20Reference) (OtherBodyIndex :type Integer) (bFromSweep :type Boolean) (SweepResult :type Hit%20Result%20Structure%20%28by%20ref%29))
  ;[1 1 1] When a character or pushable block overlaps us
  (bind _foundvalidoverlap (CallFunction|CheckValidOverlappingActors OtherActor OtherComp))
  (if _foundvalidoverlap
    (Utilities|Array|AddUnique (Variables|PressurePlate|GetOverlappingActors) OtherActor)
    ;[1 1 1] Only activate/detactive if it's the first/last person on/off the switch
    (bind _output_get (Variables|PressurePlate|SetNumberOfOverlapping (+ (Variables|PressurePlate|GetNumberOfOverlapping) 1)))
    (if (== _output_get 1)
      ;[1 1 1] Play the movement animation
      (bind (_direction _0_1) (Timeline|PressurePlateTimeline Play)
        (:Update
          (Transformation|SetRelativeLocation (Variables|Default|GetPressurePlate) (Math|Vector|MakeVector 0.0 0.0 (Math|Float|Lerp 0.0 (Variables|PressurePlate|GetPressurePlateAnimDistance) _0_1)) false false))
        (:Finished
          ;[1 1 1] Let everyone know what we're up to
          (switch Utilities|FlowControl|Switch|SwitchonETimelineDirection _direction
            (:Forward
              (if (not (Variables|PressurePlate|GetIsPressurePlateDown))
                (Variables|PressurePlate|SetIsPressurePlateDown true)
                (Default|CallOnPressurePlateActivated self)
                (else
                  (Variables|PressurePlate|SetIsPressurePlateDown true))))
            (:Backward
              (if (Variables|PressurePlate|GetIsPressurePlateDown)
                (Variables|PressurePlate|SetIsPressurePlateDown false)
                (Default|CallOnPressurePlateDeactivated self)
                (else
                  (Variables|PressurePlate|SetIsPressurePlateDown false))))))))))

(event OnComponentEndOverlap(PressurePlateCollision)
  (params (OverlappedComponent :type Primitive%20Component%20Object%20Reference) (OtherActor :type Actor%20Object%20Reference) (OtherComp :type Primitive%20Component%20Object%20Reference) (OtherBodyIndex :type Integer))
  ;[1 1 1] When a character or pushable block overlaps us
  (bind _foundvalidoverlap (CallFunction|CheckValidOverlappingActors OtherActor OtherComp))
  (if _foundvalidoverlap
    (Utilities|Array|RemoveItem (Variables|PressurePlate|GetOverlappingActors) OtherActor)
    ;[1 1 1] Only activate/detactive if it's the first/last person on/off the switch
    (bind _output_get (Variables|PressurePlate|SetNumberOfOverlapping (- (Variables|PressurePlate|GetNumberOfOverlapping) 1)))
    (if (== _output_get 0)
      ;[1 1 1] One time activation
      (if (not (Variables|PressurePlate|GetOneTimeActivation))
        ;[1 1 1] Play the movement animation
        (bind (_direction _0_1) (Timeline|PressurePlateTimeline Reverse)
          (:Update
            (Transformation|SetRelativeLocation (Variables|Default|GetPressurePlate) (Math|Vector|MakeVector 0.0 0.0 (Math|Float|Lerp 0.0 (Variables|PressurePlate|GetPressurePlateAnimDistance) _0_1)) false false))
          (:Finished
            ;[1 1 1] Let everyone know what we're up to
            (switch Utilities|FlowControl|Switch|SwitchonETimelineDirection _direction
              (:Forward
                (if (not (Variables|PressurePlate|GetIsPressurePlateDown))
                  (Variables|PressurePlate|SetIsPressurePlateDown true)
                  (Default|CallOnPressurePlateActivated self)
                  (else
                    (Variables|PressurePlate|SetIsPressurePlateDown true))))
              (:Backward
                (if (Variables|PressurePlate|GetIsPressurePlateDown)
                  (Variables|PressurePlate|SetIsPressurePlateDown false)
                  (Default|CallOnPressurePlateDeactivated self)
                  (else
                    (Variables|PressurePlate|SetIsPressurePlateDown false)))))))))))

(event Custom|test
  ;[1 1 1] Play the movement animation
  (bind (_direction _0_1) (Timeline|PressurePlateTimeline Reverse)
    (:Update
      (Transformation|SetRelativeLocation (Variables|Default|GetPressurePlate) (Math|Vector|MakeVector 0.0 0.0 (Math|Float|Lerp 0.0 (Variables|PressurePlate|GetPressurePlateAnimDistance) _0_1)) false false))
    (:Finished
      ;[1 1 1] Let everyone know what we're up to
      (switch Utilities|FlowControl|Switch|SwitchonETimelineDirection _direction
        (:Forward
          (if (not (Variables|PressurePlate|GetIsPressurePlateDown))
            (Variables|PressurePlate|SetIsPressurePlateDown true)
            (Default|CallOnPressurePlateActivated self)
            (else
              (Variables|PressurePlate|SetIsPressurePlateDown true))))
        (:Backward
          (if (Variables|PressurePlate|GetIsPressurePlateDown)
            (Variables|PressurePlate|SetIsPressurePlateDown false)
            (Default|CallOnPressurePlateDeactivated self)
            (else
              (Variables|PressurePlate|SetIsPressurePlateDown false))))))))

(event EventBeginPlay
  (bind _pressureplatecollision (Variables|Default|GetPressurePlateCollision))
  ;[1 1 1] Check if there's any overlapping actors at begin play
  (for _array_element (Collision|GetOverlappingActors _pressureplatecollision 0 :!class /Script/Engine.PrimitiveComponent)
    (for _array_element_2 (Class|PrimitiveComponent|GetOverlappingComponents _pressureplatecollision)
      (bind _foundvalidoverlap (CallFunction|CheckValidOverlappingActors _array_element _array_element_2))
      (if _foundvalidoverlap
        (Utilities|Array|AddUnique (Variables|PressurePlate|GetOverlappingActors) _array_element)
        (Components|Timeline|SetPlaybackPosition (Variables|Default|GetPressurePlateTimeline) 1.0 true true)
        ;[1 1 1] Only activate/detactive if it's the first/last person on/off the switch
        (bind _output_get (Variables|PressurePlate|SetNumberOfOverlapping (+ (Variables|PressurePlate|GetNumberOfOverlapping) 1)))
        (if (== _output_get 1)
          ;[1 1 1] Play the movement animation
          (bind (_direction _0_1) (Timeline|PressurePlateTimeline Play)
            (:Update
              (Transformation|SetRelativeLocation (Variables|Default|GetPressurePlate) (Math|Vector|MakeVector 0.0 0.0 (Math|Float|Lerp 0.0 (Variables|PressurePlate|GetPressurePlateAnimDistance) _0_1)) false false))
            (:Finished
              ;[1 1 1] Let everyone know what we're up to
              (switch Utilities|FlowControl|Switch|SwitchonETimelineDirection _direction
                (:Forward
                  (if (not (Variables|PressurePlate|GetIsPressurePlateDown))
                    (Variables|PressurePlate|SetIsPressurePlateDown true)
                    (Default|CallOnPressurePlateActivated self)
                    (else
                      (Variables|PressurePlate|SetIsPressurePlateDown true))))
                (:Backward
                  (if (Variables|PressurePlate|GetIsPressurePlateDown)
                    (Variables|PressurePlate|SetIsPressurePlateDown false)
                    (Default|CallOnPressurePlateDeactivated self)
                    (else
                      (Variables|PressurePlate|SetIsPressurePlateDown false))))))))))))

(fn ConstructionScript
  ;[1 1 1] Set the speed of the animation timeline
  (Components|Timeline|SetPlayRate (Variables|Default|GetPressurePlateTimeline) (Variables|PressurePlate|GetPressurePlatePlayRate))
  ;[1 1 1] Start with the highlight
  (CallFunction|SetActorHighlightOutline self (Variables|PressurePlate|GetBeginWithHighlightOutline)))

(fn CheckValidOverlappingActors
  (params (Actor :type Object%20Object%20Reference) (Component :type Primitive%20Component%20Object%20Reference))
  ;[1 1 1] Init vars
  (LocalVariables|SetActorLocal Actor)
  (LocalVariables|SetComponentLocal Component)
  ;[1 1 1] Comment
  (if (not (Variables|PressurePlate|GetOnlyTriggerFromPushableBlock))
    ;[1 1 1] Check if it's an object we care about
    (bind _asquest_character (Utilities|Casting|CastToQuestCharacter (LocalVariables|GetActorLocal))
      (:then
        (LocalVariables|SetFoundValidOverlapLocal (== (Variables|/Script/Engine.Character|GetCapsuleComponent _asquest_character) (LocalVariables|GetComponentLocal))))
      (:CastFailed
        (Utilities|Casting|CastToQuestDungeonPushableBlock (LocalVariables|GetActorLocal) :!label _label
          (:then
            (LocalVariables|SetFoundValidOverlapLocal true))
          (:CastFailed
            (LocalVariables|SetFoundValidOverlapLocal false)))))
    (else
      (goto _label)))
  ;[1 1 1] Return
  (return (LocalVariables|GetFoundValidOverlapLocal)))