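; Quest cemetery gate actor with two hinged leaves that the player or other logic can open, close, toggle and lock.
; A timeline rotates both hinges, swinging away from or toward a side chosen by a dot product against the player's position, then broadcasts opened or closed with a player-interacted flag.
; Interacting while locked plays a shake, and lock meshes show only while locked, shut and still.
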(event Custom|OpenGate
  ;[1 1 1] Custom events to control the door
  (Variables|Gate|SetPlayerInteracted false)
  ;[1 1 1] Comment
  (Variables|Gate|SetGateMoving true)
  (Gate|SetGateLocksVisible (Gate|GetShouldLocksbeVisible))
  ;[1 1 1] Door open animation
  (bind (_direction _0_1) (Timeline|GateOpenTimeline Play)
    (:Update
      (Transformation|SetRelativeRotation (Variables|Default|GetGateRightHinge) (Math|Rotator|MakeRotator 0.0 0.0 (Math|Float|Lerp 0.0 (* (Variables|Gate|GetGateOpenAngle) (select (Variables|Gate|GetGateOpenForward) 1.0 -1.0)) _0_1)) false false)
      (Transformation|SetRelativeRotation (Variables|Default|GetGateLeftHinge) (Math|Rotator|MakeRotator 0.0 0.0 (Math|Float|Lerp 0.0 (* (Variables|Gate|GetGateOpenAngle) (select (Variables|Gate|GetGateOpenForward) -1.0 1.0)) _0_1)) false false))
    (:Finished
      (Variables|Gate|SetGateMoving false)
      ;[1 1 1] Set the door state after the anim
      (switch Utilities|FlowControl|Switch|SwitchonETimelineDirection _direction
        (:Forward
          (Variables|Gate|SetIsGateOpen true)
          ;[1 1 1] Comment
          (Gate|SetGateLocksVisible false)
          ;[1 1 1] Tell everyone that the gate has opened
          (Default|CallGateOpened self (Variables|Gate|GetPlayerInteracted)))
        (:Backward
          (Variables|Gate|SetIsGateOpen false)
          (Gate|SetGateLocksVisible (Gate|GetShouldLocksbeVisible))
          (Default|CallGateClosed self (Variables|Gate|GetPlayerInteracted)))))))

(event Custom|CloseGate
  ;[1 1 1] Custom events to control the door
  (Variables|Gate|SetPlayerInteracted false)
  ;[1 1 1] Comment
  (Variables|Gate|SetGateMoving true)
  (Gate|SetGateLocksVisible (Gate|GetShouldLocksbeVisible))
  ;[1 1 1] Door open animation
  (bind (_direction _0_1) (Timeline|GateOpenTimeline Reverse)
    (:Update
      (Transformation|SetRelativeRotation (Variables|Default|GetGateRightHinge) (Math|Rotator|MakeRotator 0.0 0.0 (Math|Float|Lerp 0.0 (* (Variables|Gate|GetGateOpenAngle) (select (Variables|Gate|GetGateOpenForward) 1.0 -1.0)) _0_1)) false false)
      (Transformation|SetRelativeRotation (Variables|Default|GetGateLeftHinge) (Math|Rotator|MakeRotator 0.0 0.0 (Math|Float|Lerp 0.0 (* (Variables|Gate|GetGateOpenAngle) (select (Variables|Gate|GetGateOpenForward) -1.0 1.0)) _0_1)) false false))
    (:Finished
      (Variables|Gate|SetGateMoving false)
      ;[1 1 1] Set the door state after the anim
      (switch Utilities|FlowControl|Switch|SwitchonETimelineDirection _direction
        (:Forward
          (Variables|Gate|SetIsGateOpen true)
          ;[1 1 1] Comment
          (Gate|SetGateLocksVisible false)
          ;[1 1 1] Tell everyone that the gate has opened
          (Default|CallGateOpened self (Variables|Gate|GetPlayerInteracted)))
        (:Backward
          (Variables|Gate|SetIsGateOpen false)
          (Gate|SetGateLocksVisible (Gate|GetShouldLocksbeVisible))
          (Default|CallGateClosed self (Variables|Gate|GetPlayerInteracted)))))))

(event Custom|ToggleGateOpen
  ;[1 1 1] Custom events to control the door
  (Variables|Gate|SetPlayerInteracted false)
  (if (not (Variables|Gate|GetIsGateOpen))
    ;[1 1 1] Comment
    (Variables|Gate|SetGateMoving true)
    (Gate|SetGateLocksVisible (Gate|GetShouldLocksbeVisible))
    ;[1 1 1] Door open animation
    (bind (_direction _0_1) (Timeline|GateOpenTimeline Play)
      (:Update
        (Transformation|SetRelativeRotation (Variables|Default|GetGateRightHinge) (Math|Rotator|MakeRotator 0.0 0.0 (Math|Float|Lerp 0.0 (* (Variables|Gate|GetGateOpenAngle) (select (Variables|Gate|GetGateOpenForward) 1.0 -1.0)) _0_1)) false false)
        (Transformation|SetRelativeRotation (Variables|Default|GetGateLeftHinge) (Math|Rotator|MakeRotator 0.0 0.0 (Math|Float|Lerp 0.0 (* (Variables|Gate|GetGateOpenAngle) (select (Variables|Gate|GetGateOpenForward) -1.0 1.0)) _0_1)) false false))
      (:Finished
        (Variables|Gate|SetGateMoving false)
        ;[1 1 1] Set the door state after the anim
        (switch Utilities|FlowControl|Switch|SwitchonETimelineDirection _direction
          (:Forward
            (Variables|Gate|SetIsGateOpen true)
            ;[1 1 1] Comment
            (Gate|SetGateLocksVisible false)
            ;[1 1 1] Tell everyone that the gate has opened
            (Default|CallGateOpened self (Variables|Gate|GetPlayerInteracted)))
          (:Backward
            (Variables|Gate|SetIsGateOpen false)
            (Gate|SetGateLocksVisible (Gate|GetShouldLocksbeVisible))
            (Default|CallGateClosed self (Variables|Gate|GetPlayerInteracted))))))
    (else
      (Variables|Gate|SetGateMoving true)
      (Gate|SetGateLocksVisible (Gate|GetShouldLocksbeVisible))
      (Timeline|GateOpenTimeline Reverse))))

(event EventBeginPlay
  ;[1 1 1] Comment
  (if (Variables|Gate|GetOpenByDefault)
    (Components|Timeline|SetPlaybackPosition (Variables|Default|GetGateOpenTimeline) 1.0 true true)))

(event EventPlayerInteract
  ;[1 1 1] Player interacted!
  (if (not (Variables|Gate|GetLocked))
    (Variables|Gate|SetPlayerInteracted true)
    ;[1 1 1] Comment
    (if (and (not (Variables|Gate|GetGateMoving)) (not (Variables|Gate|GetIsGateOpen)))
      (Variables|Gate|SetGateOpenForward (> (Math|Vector|DotProduct (Class|KismetMathLibrary|GetDirectionVector (Transformation|GetActorLocation) (Transformation|GetActorLocation (Game|GetPlayerCharacter 0))) (Transformation|GetActorRightVector)) 0.0)))
    ;[1 1 1] Custom events to control the door
    (if (not (Variables|Gate|GetIsGateOpen))
      ;[1 1 1] Comment
      (Variables|Gate|SetGateMoving true)
      (Gate|SetGateLocksVisible (Gate|GetShouldLocksbeVisible))
      ;[1 1 1] Door open animation
      (bind (_direction _0_1) (Timeline|GateOpenTimeline Play)
        (:Update
          (Transformation|SetRelativeRotation (Variables|Default|GetGateRightHinge) (Math|Rotator|MakeRotator 0.0 0.0 (Math|Float|Lerp 0.0 (* (Variables|Gate|GetGateOpenAngle) (select (Variables|Gate|GetGateOpenForward) 1.0 -1.0)) _0_1)) false false)
          (Transformation|SetRelativeRotation (Variables|Default|GetGateLeftHinge) (Math|Rotator|MakeRotator 0.0 0.0 (Math|Float|Lerp 0.0 (* (Variables|Gate|GetGateOpenAngle) (select (Variables|Gate|GetGateOpenForward) -1.0 1.0)) _0_1)) false false))
        (:Finished
          (Variables|Gate|SetGateMoving false)
          ;[1 1 1] Set the door state after the anim
          (switch Utilities|FlowControl|Switch|SwitchonETimelineDirection _direction
            (:Forward
              (Variables|Gate|SetIsGateOpen true)
              ;[1 1 1] Comment
              (Gate|SetGateLocksVisible false)
              ;[1 1 1] Tell everyone that the gate has opened
              (Default|CallGateOpened self (Variables|Gate|GetPlayerInteracted)))
            (:Backward
              (Variables|Gate|SetIsGateOpen false)
              (Gate|SetGateLocksVisible (Gate|GetShouldLocksbeVisible))
              (Default|CallGateClosed self (Variables|Gate|GetPlayerInteracted))))))
      (else
        (Variables|Gate|SetGateMoving true)
        (Gate|SetGateLocksVisible (Gate|GetShouldLocksbeVisible))
        (Timeline|GateOpenTimeline Reverse)))
    (else
      ;[1 1 1] Shake the gate if it's locked
      (if (not (Variables|Gate|GetIsGateOpen))
        (bind _0_1_2 (Timeline|GateLockedShakeTimeline PlayFromStart)
          (:Update
            (Transformation|SetRelativeRotation (Variables|Default|GetGateRightHinge) (Math|Rotator|MakeRotator 0.0 0.0 (Math|Float|Lerp 0.0 (Variables|Gate|GetGateLockedShakeAngle) _0_1_2)) false false)
            (Transformation|SetRelativeRotation (Variables|Default|GetGateLeftHinge) (Math|Rotator|MakeRotator 0.0 0.0 (Math|Float|Lerp 0.0 (* (Variables|Gate|GetGateLockedShakeAngle) -1.0) _0_1_2)) false false)))))))

(fn ConstructionScript
  ;[1 1 1] Start with the highlight
  (CallFunction|SetActorHighlightOutline self (Variables|Gate|GetBeginWithHighlightOutline))
  (Gate|SetGateLocksVisible (and (Variables|Gate|GetLocked) (not (Variables|Gate|GetOpenByDefault)))))

(fn SetGateLocked
  (params (Locked :type Boolean :default false))
  (Variables|Gate|SetLocked Locked)
  (Gate|SetGateLocksVisible (Gate|GetShouldLocksbeVisible)))

(fn GetGateIsOpen
  ;[1 1 1] Simple function for checking gate state
  (return (Variables|Gate|GetIsGateOpen)))

(fn SetGateLocksVisible
  (params (bNewVisibility :type Boolean))
  (Rendering|SetVisibility (Variables|Default|GetLock01) bNewVisibility false))

(fn GetShouldLocksbeVisible
  (return (Math|Boolean|ANDBoolean (Variables|Gate|GetLocked) (not (Variables|Gate|GetIsGateOpen)) (not (Variables|Gate|GetGateMoving)))))

(fn GetGateLocked
  (return (Variables|Gate|GetLocked)))