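; Quest modular weapon Blueprint that assembles its visual from Head, Hilt, Handle and Pommel static meshes.
; The construction script passes the four pieces to SetModularWeaponPieces, which loops over them to add a component for each valid mesh.
; Components use manual attachment, placed with the actor's transform.
; The loop body reaches the return node on its first pass, so only Head is ever processed.
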(fn ConstructionScript
  ;[1 1 1] Set the pieces
  (CallFunction|SetModularWeaponPieces (Variables|ModularWeapon|GetHead) (Variables|ModularWeapon|GetHilt) (Variables|ModularWeapon|GetHandle) (Variables|ModularWeapon|GetPommel)))

(fn SetModularWeaponPieces
  (params (Head :type Static%20Mesh%20Object%20Reference) (Hilt :type Static%20Mesh%20Object%20Reference) (Handle :type Static%20Mesh%20Object%20Reference) (Pommel :type Static%20Mesh%20Object%20Reference))
  ;[1 1 1] Create the modular weapon
  (for _array_element (Utilities|Array|MakeArray Head Hilt Handle Pommel)
    (Utilities|IsValid _array_element
      (:Is%20Valid
        (bind _returnvalue (AddComponent|AddStaticMeshComponent true (Transformation|GetActorTransform)))
        (Components|StaticMesh|SetStaticMesh _returnvalue _array_element))
      (:Is%20Not%20Valid
        _))
    (return true))
  (return true))