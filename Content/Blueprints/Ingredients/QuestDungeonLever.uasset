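; Dungeon lever that flips between two pitch rotations, either by player interaction or by an external FlipLever event.
; A timeline animates the rotation forward or backward, then updates the flipped state and calls OnLeverFlipped with direction and whether the player triggered it.
; Only player interaction respects the lock, which can engage automatically after the first flip.
; Instance variables set the default flipped state and starting highlight outline.
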(event Custom|FlipLever
  ;[1 1 1] Recieve event to flip (╯°□°)╯︵ ┻━┻
  ;[1 1 1] Make sure we're not locked
  (Variables|Lever|SetPlayerInteracted false)
  ;[1 1 1] Which way?
  (if (not (Variables|Lever|GetLeverIsFlipped))
    ;[1 1 1] Animation timeline: Rotate the lever
    (bind (_direction _0_1) (Timeline|FlipLeverTimeline Play)
      (:Update
        (Transformation|SetRelativeRotation (Variables|Default|GetLeverBase) (Math|Rotator|MakeRotator 0.0 (Math|Float|Lerp (Variables|Lever|GetLeverInitialRotation) (Variables|Lever|GetLeverFinalRotation) _0_1) 0.0) false false))
      (:Finished
        ;[1 1 1] Let the world know we flipped
        (switch Utilities|FlowControl|Switch|SwitchonETimelineDirection _direction
          (:Forward
            (Variables|Lever|SetLeverIsFlipped true))
          (:Backward
            (Variables|Lever|SetLeverIsFlipped false)))
        (Default|CallOnLeverFlipped _direction (Variables|Lever|GetPlayerInteracted))
        ;[1 1 1] Lock after the first use
        (bind _result (Math|Integer|IncrementInt (Variables|Lever|GetTimesFlipped))
          (:%20%20
            (if (and (== _result 1) (Variables|Lever|GetAutoLockAfterFirstUse))
              (Lever|SetLeverLocked true))))))
    (else
      (Timeline|FlipLeverTimeline Reverse))))

(event EventBeginPlay
  ;[1 1 1] Check if we start flipped or not
  (if (Variables|Lever|GetFlippedByDefault)
    (Components|Timeline|SetPlaybackPosition (Variables|Default|GetFlipLeverTimeline) 1.0 true true)))

(event EventPlayerInteract
  ;[1 1 1] Recieve event to flip (╯°□°)╯︵ ┻━┻
  ;[1 1 1] Make sure we're not locked
  (if (not (Variables|Lever|GetLocked))
    (Variables|Lever|SetPlayerInteracted true)
    ;[1 1 1] Which way?
    (if (not (Variables|Lever|GetLeverIsFlipped))
      ;[1 1 1] Animation timeline: Rotate the lever
      (bind (_direction _0_1) (Timeline|FlipLeverTimeline Play)
        (:Update
          (Transformation|SetRelativeRotation (Variables|Default|GetLeverBase) (Math|Rotator|MakeRotator 0.0 (Math|Float|Lerp (Variables|Lever|GetLeverInitialRotation) (Variables|Lever|GetLeverFinalRotation) _0_1) 0.0) false false))
        (:Finished
          ;[1 1 1] Let the world know we flipped
          (switch Utilities|FlowControl|Switch|SwitchonETimelineDirection _direction
            (:Forward
              (Variables|Lever|SetLeverIsFlipped true))
            (:Backward
              (Variables|Lever|SetLeverIsFlipped false)))
          (Default|CallOnLeverFlipped _direction (Variables|Lever|GetPlayerInteracted))
          ;[1 1 1] Lock after the first use
          (bind _result (Math|Integer|IncrementInt (Variables|Lever|GetTimesFlipped))
            (:%20%20
              (if (and (== _result 1) (Variables|Lever|GetAutoLockAfterFirstUse))
                (Lever|SetLeverLocked true))))))
      (else
        (Timeline|FlipLeverTimeline Reverse)))))

(fn ConstructionScript
  ;[1 1 1] Set the initial position based on variables
  (Transformation|SetRelativeRotation (Variables|Default|GetLeverBase) (Math|Rotator|MakeRotator 0.0 (Variables|Lever|GetLeverInitialRotation) 0.0) false false)
  ;[1 1 1] Set its default value
  (Variables|Lever|SetLeverIsFlipped (Variables|Lever|GetFlippedByDefault))
  ;[1 1 1] Start with the highlight
  (CallFunction|SetActorHighlightOutline self (Variables|Lever|GetBeginWithHighlightOutline)))

(fn SetLeverLocked
  (params (Locked :type Boolean :default false))
  (Variables|Lever|SetLocked Locked))

(fn GetLeverLocked
  (return (Variables|Lever|GetLocked)))