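; Quest loot pickup that becomes a potion, gold, key or gem, with its mesh and optional highlight set in the construction script.
; On QuestCharacter_Juno overlap, potions heal by strength regardless of potion type, only below max health, while gold and keys update inventory.
; Successful pickups, including gems which grant nothing here, fire OnPickupAcquired and self-destruct.
; Grow and bounce timelines are unwired, and RotateToCamera is never called here.
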(event OnComponentBeginOverlap(PickupCollision)
  (params (OtherActor :type Actor%20Object%20Reference) (OtherComp :type Primitive%20Component%20Object%20Reference) (OtherBodyIndex :type Integer) (bFromSweep :type Boolean) (SweepResult :type Hit%20Result%20Structure%20%28by%20ref%29))
  ;[1 1 1] Player walks into the pickup
  (bind _asquest_character_juno (Utilities|Casting|CastToQuestCharacter_Juno OtherActor))
  (Variables|Pickup|SetPlayerCharacter _asquest_character_juno)
  ;[1 1 1] Which item is this?
  (switch Utilities|FlowControl|Switch|SwitchonEnum_PickupTypes (Variables|Pickup|GetPickupType)
    (:NewEnumerator0
      ;[1 1 1] Prevent the player from snagging this sweet treat if they already full
      (if (< (Variables|/Game/Blueprints/Characters/QuestCharacter.QuestCharacter_C|GetHealth (Variables|Pickup|GetPlayerCharacter)) (Variables|/Game/Blueprints/Characters/QuestCharacter.QuestCharacter_C|GetMaxHealth (Variables|Pickup|GetPlayerCharacter)))
        ;[1 1 1] How much do we heal for?
        (Variables|Pickup|SetHealAmount (Utilities|Select :Index (Variables|Pickup|GetPotionStrength) :NewEnumerator2 (Variables|Pickup|GetHealAmountMinor) :NewEnumerator1 (Variables|Pickup|GetHealAmountMedium) :NewEnumerator0 (Variables|Pickup|GetHealAmountLarge) :NewEnumerator3 (Variables|Pickup|GetHealAmountEpic)))
        ;[1 1 1] Health
        (Default|UpdateHealth (Variables|Pickup|GetPlayerCharacter) "NewEnumerator1" (Variables|Pickup|GetHealAmount))
        ;[1 1 1] Call the dispatcher and then self destruct!
        (Default|CallOnPickupAcquired self :!label _label)
        (Actor|DestroyActor)))
    (:NewEnumerator1
      ;[1 1 1] Gold
      (Default|UpdateInventory (Variables|Pickup|GetPlayerCharacter) "NewEnumerator0" "NewEnumerator0" (Variables|Pickup|GetGoldAmount))
      (goto _label))
    (:NewEnumerator2
      ;[1 1 1] Key
      (Default|UpdateInventory (Variables|Pickup|GetPlayerCharacter) "NewEnumerator0" "NewEnumerator1" (Variables|Pickup|GetKeyAmount))
      (goto _label))
    (:NewEnumerator4
      (goto _label))))

(fn ConstructionScript
  ;[1 1 1] Set the mesh
  (CallFunction|SetPickupMesh)
  ;[1 1 1] Store the mesh's intial location
  (Variables|Pickup|SetPickupBounceStartPosition (Variables|/Script/Engine.SceneComponent|GetRelativeLocation (Variables|Default|GetPickupMesh)))
  ;[1 1 1] Highlight the object
  (CallFunction|SetActorHighlightOutline self (Variables|Pickup|GetBeginWithHighlight)))

(fn RotatetoCamera
  (bind _returnvalue (Game|GetPlayerCameraManager 0))
  (Utilities|IsValid _returnvalue
    (:Is%20Valid
      (Transformation|SetWorldRotation (Variables|Default|GetPickupMesh) (Math|Rotator|MakeRotator 0.0 0.0 (+ (.Yaw (Math|Rotator|BreakRotator (Math|Rotator|FindLookatRotation (Transformation|GetActorLocation) (Transformation|GetActorLocation _returnvalue)))) 1.8e+02)) false false))
    (:Is%20Not%20Valid
      _))
  (return))

(fn SetPickupMesh
  (switch Utilities|FlowControl|Switch|SwitchonEnum_PickupTypes (Variables|Pickup|GetPickupType)
    (:NewEnumerator0
      ;[1 1 1] Set potion model
      (switch Utilities|FlowControl|Switch|SwitchonEnum_PotionAffectTypes (Variables|Pickup|GetPotionType)
        (:NewEnumerator0
          (Variables|Pickup|SetMeshToUse (Utilities|Select :Index (Variables|Pickup|GetPotionStrength) :NewEnumerator2 "/Game/Props/Loot/Meshes/PropLoot_PotionMinor_Red.PropLoot_PotionMinor_Red" :NewEnumerator1 "/Game/Props/Loot/Meshes/PropLoot_PotionMedium_Red.PropLoot_PotionMedium_Red" :NewEnumerator0 "/Game/Props/Loot/Meshes/PropLoot_PotionLarge_Red.PropLoot_PotionLarge_Red" :NewEnumerator3 "/Game/Props/Loot/Meshes/PropLoot_PotionEpic_Red.PropLoot_PotionEpic_Red")))
        (:NewEnumerator2
          (Variables|Pickup|SetMeshToUse (Utilities|Select :Index (Variables|Pickup|GetPotionStrength) :NewEnumerator2 "/Game/Props/Loot/Meshes/PropLoot_PotionMinor_Blue.PropLoot_PotionMinor_Blue" :NewEnumerator1 "/Game/Props/Loot/Meshes/PropLoot_PotionMedium_Blue.PropLoot_PotionMedium_Blue" :NewEnumerator0 "/Game/Props/Loot/Meshes/PropLoot_PotionLarge_Blue.PropLoot_PotionLarge_Blue" :NewEnumerator3 "/Game/Props/Loot/Meshes/PropLoot_PotionEpic_Blue.PropLoot_PotionEpic_Blue")))
        (:NewEnumerator3
          (Variables|Pickup|SetMeshToUse (Utilities|Select :Index (Variables|Pickup|GetPotionStrength) :NewEnumerator2 "/Game/Props/Loot/Meshes/PropLoot_PotionMinor_Purple.PropLoot_PotionMinor_Purple" :NewEnumerator1 "/Game/Props/Loot/Meshes/PropLoot_PotionMedium_Purple.PropLoot_PotionMedium_Purple" :NewEnumerator0 "/Game/Props/Loot/Meshes/PropLoot_PotionLarge_Purple.PropLoot_PotionLarge_Purple" :NewEnumerator3 "/Game/Props/Loot/Meshes/PropLoot_PotionEpic_Purple.PropLoot_PotionEpic_Purple")))
        (:NewEnumerator1
          (Variables|Pickup|SetMeshToUse (Utilities|Select :Index (Variables|Pickup|GetPotionStrength) :NewEnumerator2 "/Game/Props/Loot/Meshes/PropLoot_PotionMinor_Green.PropLoot_PotionMinor_Green" :NewEnumerator1 "/Game/Props/Loot/Meshes/PropLoot_PotionMedium_Green.PropLoot_PotionMedium_Green" :NewEnumerator0 "/Game/Props/Loot/Meshes/PropLoot_PotionLarge_Green.PropLoot_PotionLarge_Green" :NewEnumerator3 "/Game/Props/Loot/Meshes/PropLoot_PotionEpic_Green.PropLoot_PotionEpic_Green")))))
    (:NewEnumerator1
      ;[1 1 1] Set gold mesh
      (Variables|Pickup|SetMeshToUse "/Game/Props/Loot/Meshes/PropLoot_SackOfGold_Small01.PropLoot_SackOfGold_Small01"))
    (:NewEnumerator2
      ;[1 1 1] Set key type
      (Variables|Pickup|SetMeshToUse (Utilities|Select :Index (Variables|Pickup|GetKeyType) :NewEnumerator0 "/Game/Props/Loot/Meshes/PropLoot_Key_Silver.PropLoot_Key_Silver" :NewEnumerator1 "/Game/Props/Loot/Meshes/PropLoot_Key_Gold.PropLoot_Key_Gold"))
      (Transformation|AddRelativeRotation (Variables|Default|GetPickupMesh) "-90.000000, 0, 0" false false))
    (:NewEnumerator4
      ;[1 1 1] Set gem type
      (Variables|Pickup|SetMeshToUse (Utilities|Select :Index (Variables|Pickup|GetGemType) :NewEnumerator0 "/Game/Props/Loot/Meshes/PropLoot_Gem_Amethyst.PropLoot_Gem_Amethyst" :NewEnumerator1 "/Game/Props/Loot/Meshes/PropLoot_Gem_Topaz.PropLoot_Gem_Topaz" :NewEnumerator2 "/Game/Props/Loot/Meshes/PropLoot_Gem_Emerald.PropLoot_Gem_Emerald" :NewEnumerator3 "/Game/Props/Loot/Meshes/PropLoot_Gem_Sapphire.PropLoot_Gem_Sapphire" :NewEnumerator4 "/Game/Props/Loot/Meshes/PropLoot_Gem_Ruby.PropLoot_Gem_Ruby" :NewEnumerator5 "/Game/Props/Loot/Meshes/PropLoot_Gem_Diamond.PropLoot_Gem_Diamond"))))
  ;[1 1 1] Set the model
  (Components|StaticMesh|SetStaticMesh (Variables|Default|GetPickupMesh) (Variables|Pickup|GetMeshToUse))
  (return))