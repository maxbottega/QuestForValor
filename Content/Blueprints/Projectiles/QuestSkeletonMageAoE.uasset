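; Skeleton mage area-of-effect attack that strikes at the feet of the instigator's target.
; The construction script reads CurrentTarget from the instigator's AI Blackboard and moves the actor to that character's capsule base.
; On BeginPlay it plays a start effect, waits, plays an end effect, then capsule-traces for unique actors.
; QuestCharacters other than the instigator take damage, gated by a faction-standing check, before the actor self-destructs after its lifetime.
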(event EventBeginPlay
  (bind _returnvalue (Transformation|GetActorLocation))
  (bind _returnvalue_2 (Transformation|GetActorLocation))
  (Effects|SpawnEmitteratLocation "/Game/Effects/Particles/Systems/P_AOE_MageAOE_Start.P_AOE_MageAOE_Start" _returnvalue)
  (Utilities|FlowControl|Delay (Variables|Default|GetDamageDelay))
  (Effects|SpawnEmitteratLocation "/Game/Effects/Particles/Systems/P_AOE_MageAOE_End.P_AOE_MageAOE_End" _returnvalue)
  (bind _outhits (Class|KismetSystemLibrary|CapsuleTraceMultiforObjects _returnvalue_2 (+ _returnvalue_2 "0, 0,1.000000") (Variables|Default|GetRadius) (Variables|Default|GetHalfHeight) (Utilities|Array|MakeArray "ObjectTypeQuery3" "ObjectTypeQuery2" "ObjectTypeQuery6") false 0 "None" true))
  (for _array_element _outhits
    (Utilities|Array|AddUnique (Variables|Default|GetHitActors) (.HitActor (Collision|BreakHitResult _array_element))))
  (for _array_element_2 (Variables|Default|GetHitActors)
    (bind _asquest_character (Utilities|Casting|CastToQuestCharacter _array_element_2))
    (Variables|Default|SetCharacterHit _asquest_character)
    (if (!= (Variables|Default|GetCharacterHit) (Game|GetInstigator))
      (bind _asquest_character_2 (Utilities|Casting|CastToQuestCharacter (Game|GetInstigator))
        (:then
          (bind _ishostile (Default|CheckCharacterFactionStanding _asquest_character_2 (Variables|Default|GetCharacterHit)))
          (if _ishostile
            (Game|Damage|ApplyDamage (Variables|Default|GetCharacterHit) (Variables|Default|GetProjectileDamage) (Pawn|GetController (Game|GetInstigator)) self (Variables|Default|GetProjectDamageTypeClass) :!label _label)))
        (:CastFailed
          (goto _label)))))
  (Utilities|FlowControl|Delay (Variables|Default|GetLifetime))
  (Actor|DestroyActor))

(fn ConstructionScript
  (bind _returnvalue (Game|GetInstigatorController))
  ;[1 1 1] Find our target
  (Utilities|IsValid _returnvalue
    (:Is%20Valid
      (Variables|Default|SetTarget (.AsActor (Utilities|Casting|CastToActor (AI|Components|Blackboard|GetValueasObject (AI|GetBlackboard _returnvalue) (Utilities|Name|MakeLiteralName "CurrentTarget")))))
      (bind _ascharacter (Utilities|Casting|CastToCharacter (Variables|Default|GetTarget))
        (:then
          _)
        (:CastFailed
          _))
      ;[1 1 1] Move us to the target
      (Transformation|SetActorLocation (Math|Vector|MakeVector (.X (Math|Vector|BreakVector (Transformation|GetActorLocation (Variables|Default|GetTarget)))) (.Y (Math|Vector|BreakVector (Transformation|GetActorLocation (Variables|Default|GetTarget)))) (- (.Z (Math|Vector|BreakVector (Transformation|GetActorLocation (Variables|Default|GetTarget)))) (Components|Capsule|GetScaledCapsuleHalfHeight (Variables|/Script/Engine.Character|GetCapsuleComponent _ascharacter)))) false false))))