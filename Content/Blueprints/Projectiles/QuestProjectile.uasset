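; Projectile actor for quest characters that damages characters it overlaps, optionally homing on its instigator's current target.
; At BeginPlay, homing sets the movement component's target and acceleration, and a lifetime delay schedules destruction.
; Overlaps ignore the instigator and apply damage after a faction standing check, skipped for non-character instigators, then destroy the projectile.
; Blocking hits also destroy it, spawning an optional destruction particle.
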(event OnComponentHit(ProjectileCollision)
  (params (HitComponent :type Primitive%20Component%20Object%20Reference) (OtherActor :type Actor%20Object%20Reference) (OtherComp :type Primitive%20Component%20Object%20Reference) (NormalImpulse :type Vector :default "0, 0, 0") (Hit :type Hit%20Result%20Structure%20%28by%20ref%29))
  ;[1 1 1] Destroy ourselves!
  (CallFunction|DestroyProjectile))

(event OnComponentBeginOverlap(ProjectileCollision)
  (params (OverlappedComponent :type Primitive%20Component%20Object%20Reference) (OtherActor :type Actor%20Object%20Reference) (OtherComp :type Primitive%20Component%20Object%20Reference) (OtherBodyIndex :type Integer) (bFromSweep :type Boolean) (SweepResult :type Hit%20Result%20Structure%20%28by%20ref%29))
  ;[1 1 1] We hit something, check if it's the player
  (bind _asquest_character (Utilities|Casting|CastToQuestCharacter OtherActor))
  (Variables|Default|SetCharacterHit _asquest_character)
  ;[1 1 1] Make sure it's not ourselves
  (if (!= (Variables|Default|GetCharacterHit) (Game|GetInstigator))
    ;[1 1 1] Only damage if it's an enemy
    (bind _asquest_character_2 (Utilities|Casting|CastToQuestCharacter (Game|GetInstigator))
      (:then
        (bind _ishostile (Default|CheckCharacterFactionStanding _asquest_character_2 (Variables|Default|GetCharacterHit)))
        (if _ishostile
          ;[1 1 1] Damage away!
          (Game|Damage|ApplyDamage (Variables|Default|GetCharacterHit) (Variables|Default|GetProjectileDamage) (Pawn|GetController (Game|GetInstigator)) self (Variables|Default|GetProjectDamageTypeClass) :!label _label)
          ;[1 1 1] Destroy ourselves
          (CallFunction|DestroyProjectile)))
      (:CastFailed
        (goto _label)))))

(event Custom|DestroyProjectile
  ;[1 1 1] Handle the destruction of this actor
  (Utilities|IsValid (Variables|Default|GetDestructionParticle)
    (:Is%20Valid
      (Effects|SpawnEmitteratLocation (Variables|Default|GetDestructionParticle) (Transformation|GetActorLocation))
      (Utilities|FlowControl|Delay 0.0)
      (Actor|DestroyActor))
    (:Is%20Not%20Valid
      (Actor|DestroyActor))))

(event EventBeginPlay
  ;[1 1 1] Begin play!
  ;[1 1 1] Get the current target if there is one
  (if (Variables|Default|GetIsHoming)
    (bind _asquest_character (Utilities|Casting|CastToQuestCharacter (Variables|Actor|GetInstigator)))
    (bind _output_get (Variables|Default|SetCurrentTarget (Variables|/Game/Blueprints/Characters/QuestCharacter.QuestCharacter_C|GetCurrentTarget _asquest_character)))
    (Utilities|IsValid _output_get
      (:Is%20Valid
        (CallFunction|SetHomingTarget (Variables|Default|GetCurrentTarget)))
      (:Is%20Not%20Valid
        _)))
  ;[1 1 1] Set a life time so they don't hang around forever
  (Utilities|FlowControl|Delay (Variables|Default|GetProjectileLifeTime))
  (CallFunction|DestroyProjectile))

(fn ConstructionScript)

(fn SetHomingTarget
  (params (HomingTarget :type Actor%20Object%20Reference))
  (Variables|/Script/Engine.ProjectileMovementComponent|SetHomingTargetComponent (Variables|Default|GetProjectileMovement) (VehicleSound|GetRootComponent HomingTarget))
  (Variables|/Script/Engine.ProjectileMovementComponent|SetbIsHomingProjectile (Variables|Default|GetProjectileMovement) true)
  (Variables|/Script/Engine.ProjectileMovementComponent|SetHomingAccelerationMagnitude (Variables|Default|GetProjectileMovement) (Variables|Default|GetHomingStrength)))