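; Blueprint library for quest dialogue that creates a dialogue box on a speaking actor.
; CreateDialogueBox spawns a QuestDialogueBox actor at the speaker's location with the given text, ignoring collisions.
; It snaps the box to the speaker as an attachment, shifts it by a relative offset and returns it to the caller.
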(fn CreateDialogueBox
  (params (DialogueSpeaker :type Actor%20Object%20Reference) (DialogueBoxOffset :type Vector :default "0,0,180") (DialogueText :type Text))
  ;[1 1 1] Init vars
  (LocalVariables|SetDialogueSpeakerLocal DialogueSpeaker)
  (LocalVariables|SetDialogueBoxOffsetLocal DialogueBoxOffset)
  (LocalVariables|SetTextLocal DialogueText)
  ;[1 1 1] Create the widget
  (bind _returnvalue (Game|SpawnActorfromClass "/Game/UI/Blueprints/QuestDialogueBox.QuestDialogueBox_C" (Math|Transform|MakeTransform (Transformation|GetActorLocation (LocalVariables|GetDialogueSpeakerLocal)) "0, 0, 0" "1.000000,1.000000,1.000000") "AlwaysSpawn" 0 (LocalVariables|GetTextLocal) 0))
  (LocalVariables|SetCurrentDialogueBox _returnvalue)
  ;[1 1 1] Attach to papa actor
  (Class|Actor|AttachRootComponenttoActor (LocalVariables|GetCurrentDialogueBox) (LocalVariables|GetDialogueSpeakerLocal) "None" "SnapToTarget" true)
  ;[1 1 1] Add a relative offset
  (Transformation|AddRelativeLocation (LocalVariables|GetCurrentDialogueBox) (LocalVariables|GetDialogueBoxOffsetLocal) false false)
  ;[1 1 1] Return with the var
  (return (LocalVariables|GetCurrentDialogueBox)))