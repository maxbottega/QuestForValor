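; Blueprint function library of gameplay helpers for quest markers, GSR key-value storage and cinematic input locking.
; GSR get and set calls and marker lookups go through messages to the Game Instance, with GSR access fixed to one cell.
; If no markers are returned, the lookup calls SetMarkerActive(false) on the first QuestMarker actor and retries.
; The cinematic toggle disables or re-enables input on the first player's character.
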(fn FGetActiveQuestMarker
  (bind _activemarkers (Class|QuestMarkerInterface|GetMarkers(Message) (Game|GetGameInstance) :!label _label))
  (if (> (Utilities|Array|Length _activemarkers) 0)
    (return (Utilities|Array|Get(acopy) _activemarkers))
    (else
      (bind _outactors (Actor|GetAllActorsOfClass 0 "/Game/Blueprints/Ingredients/QuestMarker.QuestMarker_C"))
      (Default|SetMarkerActive (Utilities|Array|Get(acopy) _outactors) false)
      (goto _label))))

(fn FGetGSR
  (params (GSRKey :type Name))
  (bind _gsrvalue (Class|GSRInterface|GetGSR(Message) (Game|GetGameInstance) "NewEnumerator0" GSRKey))
  (return _gsrvalue))

(fn FSetGSR
  (params (GSRKey :type Name) (GSRValue :type Integer))
  (Class|GSRInterface|SetGSR(Message) (Game|GetGameInstance) "NewEnumerator0" GSRKey GSRValue))

(fn FToggleCinematicStance
  (params (isCharacterLockedDown :type Boolean))
  (bind _returnvalue (Game|GetPlayerController 0))
  (bind _returnvalue_2 (Game|GetPlayerCharacter 0))
  (if isCharacterLockedDown
    (Input|DisableInput _returnvalue_2 _returnvalue)
    (else
      (Input|EnableInput _returnvalue_2 _returnvalue))))