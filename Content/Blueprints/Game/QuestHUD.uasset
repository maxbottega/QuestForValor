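; QuestHUD is a HUD Blueprint that draws floating on-screen labels for quest objective markers.
; Each frame, DrawHUD gets the marker list from the Game Instance, projects each valid marker's location to screen space, and skips those behind the camera.
; Visible markers get an orange label with the marker type and distance to the player in meters, centered using measured text width and offset slightly upward.
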(event EventDrawHUD
  (params (SizeX :type Integer) (SizeY :type Integer))
  (bind _activemarkers (Class|QuestMarkerInterface|GetMarkers(Message) (Game|GetGameInstance)))
  (for _array_element _activemarkers
    (Variables|Default|SetCurrentMarkerIndex _array_element)
    ;[1 1 1] Objective and player
    (if (and (Utilities|IsValid (Variables|Default|GetCurrentMarkerIndex)) (Utilities|IsValid (Game|GetPlayerCharacter 0)))
      (if (> (.Z (Math|Vector|BreakVector (Class|HUD|Project (Transformation|GetActorLocation (Variables|Default|GetCurrentMarkerIndex))))) 0.0) ; Only proceed if the objective is in front of the player
        (HUD|DrawText (Utilities|String|Append (Utilities|String|EnumtoString (Default|GetMarkerType (Variables|Default|GetCurrentMarkerIndex))) (Utilities|String|Append (Utilities|String|Append ": " (Utilities|String|ToString(Integer) (Math|Float|Round (/ (Math|Vector|VectorLength (- (Transformation|GetActorLocation (Game|Player|GetPlayerPawn 0)) (Transformation|GetActorLocation (Variables|Default|GetCurrentMarkerIndex)))) 1e+02)))) "m")) "(R=1.000000,G=0.425069,B=0.000000,A=1.000000)" (- (.X (Math|Vector|BreakVector (Class|HUD|Project (Transformation|GetActorLocation (Variables|Default|GetCurrentMarkerIndex))))) (/ (.OutWidth (Class|HUD|GetTextSize (Utilities|String|Append (Utilities|String|EnumtoString (Default|GetMarkerType (Variables|Default|GetCurrentMarkerIndex))) (Utilities|String|Append (Utilities|String|Append ": " (Utilities|String|ToString(Integer) (Math|Float|Round (/ (Math|Vector|VectorLength (- (Transformation|GetActorLocation (Game|Player|GetPlayerPawn 0)) (Transformation|GetActorLocation (Variables|Default|GetCurrentMarkerIndex)))) 1e+02)))) "m")) "/Game/UI/Fonts/Font_Almendra-Regular.Font_Almendra-Regular" 1.0)) 2.0)) (- (.Y (Math|Vector|BreakVector (Class|HUD|Project (Transformation|GetActorLocation (Variables|Default|GetCurrentMarkerIndex))))) 5e+01) "/Game/UI/Fonts/Font_Almendra-Regular.Font_Almendra-Regular" 1.0 false) ; Draw text at the specified screen coordinates
      ))))

(fn ConstructionScript)