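; QuestGameState is a game state that groups AI controllers into named squads, split into melee and ranged by character role.
; AddToSquad updates or creates a squad; creation also calls ReevaluateActiveInSquad and sets it on a randomized looping timer.
; That function rewrites each squad's active lists, but its random melee attack-token selection is disconnected.
; Tick is empty, with squad debug drawing left unwired.
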(event EventTick
  (params (DeltaSeconds :type Float%20%28single-precision%29)))

(fn ConstructionScript)

(fn AddtoSquad
  (params (SquadName :type Name) (Controller :type Controller%20Object%20Reference))
  (LocalVariables|SetSquadNameLocal SquadName)
  (LocalVariables|SetControllerLocal Controller)
  (bind (_array_element _array_index) (Utilities|Array|ForEachLoopwithBreak (Variables|Default|GetSquads))
    (:LoopBody
      (LocalVariables|SetCurrentIndexLocal _array_index)
      (if (Utilities|Name|Equal(Name) (.SquadName (Utilities|Struct|BreakStruct_Squad _array_element)) (LocalVariables|GetSquadNameLocal))
        (LocalVariables|SetSquadExists true)
        ;[1 1 1] Comment
        (LocalVariables|SetSquadAIMeleeTotal (.SquadAIMeleeTotal (Utilities|Struct|BreakStruct_Squad (Utilities|Array|Get(acopy) (Variables|Default|GetSquads) (LocalVariables|GetCurrentIndexLocal)))))
        (LocalVariables|SetSquadAIRangedTotal (.SquadAIRangedTotal (Utilities|Struct|BreakStruct_Squad (Utilities|Array|Get(acopy) (Variables|Default|GetSquads) (LocalVariables|GetCurrentIndexLocal)))))
        ;[1 1 1] Comment
        (switch Utilities|FlowControl|Switch|SwitchonEnum_Role (Variables|/Game/Blueprints/Characters/QuestCharacter.QuestCharacter_C|GetCharacterRole (.AsQuest%20Character (Utilities|Casting|CastToQuestCharacter (Pawn|GetControlledPawn (LocalVariables|GetControllerLocal)))))
          (:NewEnumerator0
            (Utilities|Array|AddUnique (LocalVariables|GetSquadAIMeleeTotal) (LocalVariables|GetControllerLocal)))
          (:NewEnumerator1
            (Utilities|Array|AddUnique (LocalVariables|GetSquadAIRangedTotal) (LocalVariables|GetControllerLocal))))
        ;[1 1 1] Comment
        (Utilities|Array|SetArrayElem (Variables|Default|GetSquads) (LocalVariables|GetCurrentIndexLocal) (Utilities|Struct|MakeStruct_Squad (.SquadName (Utilities|Struct|BreakStruct_Squad (Utilities|Array|Get(acopy) (Variables|Default|GetSquads) (LocalVariables|GetCurrentIndexLocal)))) (.NumActiveMeleeTokens (Utilities|Struct|BreakStruct_Squad (Utilities|Array|Get(acopy) (Variables|Default|GetSquads) (LocalVariables|GetCurrentIndexLocal)))) (LocalVariables|GetSquadAIMeleeTotal) (.SquadAIMeleeActive (Utilities|Struct|BreakStruct_Squad (Utilities|Array|Get(acopy) (Variables|Default|GetSquads) (LocalVariables|GetCurrentIndexLocal)))) (.NumActiveRangedTokens (Utilities|Struct|BreakStruct_Squad (Utilities|Array|Get(acopy) (Variables|Default|GetSquads) (LocalVariables|GetCurrentIndexLocal)))) (LocalVariables|GetSquadAIRangedTotal) (.SquadAIRangedActive (Utilities|Struct|BreakStruct_Squad (Utilities|Array|Get(acopy) (Variables|Default|GetSquads) (LocalVariables|GetCurrentIndexLocal))))) true)))
    (:Completed
      (if (not (LocalVariables|GetSquadExists))
        ;[1 1 1] Comment
        (switch Utilities|FlowControl|Switch|SwitchonEnum_Role (Variables|/Game/Blueprints/Characters/QuestCharacter.QuestCharacter_C|GetCharacterRole (.AsQuest%20Character (Utilities|Casting|CastToQuestCharacter (Pawn|GetControlledPawn (LocalVariables|GetControllerLocal)))))
          (:NewEnumerator0
            (Utilities|Array|AddUnique (LocalVariables|GetSquadAIMeleeTotal) (LocalVariables|GetControllerLocal)))
          (:NewEnumerator1
            (Utilities|Array|AddUnique (LocalVariables|GetSquadAIRangedTotal) (LocalVariables|GetControllerLocal))))
        (Utilities|Array|AddUnique (Variables|Default|GetSquads) (Utilities|Struct|MakeStruct_Squad (LocalVariables|GetSquadNameLocal) 1 (LocalVariables|GetSquadAIMeleeTotal) (Utilities|Array|MakeArray 0) 1 (LocalVariables|GetSquadAIRangedTotal) (Utilities|Array|MakeArray 0)))
        (CallFunction|ReevaluateActiveinSquad)
        (Utilities|Time|SetTimerbyFunctionName self "ReevaluateActiveInSquad" (Math|Random|RandomFloatinRange 8.0 12.0) true)))))

(fn ReevaluateActiveinSquad
  (for (_array_element _array_index) (Variables|Default|GetSquads)
    (Utilities|Array|SetArrayElem (Variables|Default|GetSquads) _array_index (Utilities|Struct|MakeStruct_Squad (.SquadName (Utilities|Struct|BreakStruct_Squad _array_element)) (.NumActiveMeleeTokens (Utilities|Struct|BreakStruct_Squad _array_element)) (.SquadAIMeleeTotal (Utilities|Struct|BreakStruct_Squad _array_element)) (LocalVariables|GetActiveMelee) (.NumActiveRangedTokens (Utilities|Struct|BreakStruct_Squad _array_element)) (.SquadAIRangedTotal (Utilities|Struct|BreakStruct_Squad _array_element)) (LocalVariables|GetActiveRanged)) true)))