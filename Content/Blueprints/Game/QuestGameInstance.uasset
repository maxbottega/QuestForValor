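; Quest game instance that holds checkpoint, quest marker and GSR state, and pushes journal text to the player HUD.
; Checkpoints are saved as PlayerStart tags, defaulting to Checkpoint_01, and resolved by scanning level PlayerStarts; the lookup ignores its tag argument and matches the current tag.
; GSR is an array of value entries keyed by cell and key, updated in place or appended.
; SetJournal reaches the HUD through QuestGameMode and opens the journal.
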(fn FindPlayerStartbyTag
  (params (PlayerStartTagToSearch :type Name))
  (LocalVariables|SetPlayerStartTagToSearchLocal PlayerStartTagToSearch)
  (bind _outactors (Actor|GetAllActorsOfClass "/Script/Engine.PlayerStart"))
  (for _array_element _outactors
    (if (Utilities|Name|Equal(Name) (Variables|/Script/Engine.PlayerStart|GetPlayerStartTag _array_element) (Variables|Default|GetCurrentPlayerStartTag))
      (LocalVariables|SetCurrentPlayerStartLocal _array_element)
      (LocalVariables|SetFoundPlayerStartLocal true)))
  (return (LocalVariables|GetCurrentPlayerStartLocal) (LocalVariables|GetFoundPlayerStartLocal)))

(fn ClearMarker
  (params (Marker :type Quest%20Marker%20Object%20Reference))
  (Utilities|IsValid Marker
    (:Is%20Valid
      (Utilities|Array|RemoveItem (Variables|Default|GetQuestMarkers) Marker)
      (return true))
    (:Is%20Not%20Valid
      (return false))))

(fn GetCurrentCheckpoint
  ;[1 1 1] Return the correct player start based off it's tag
  (bind _playerstart (CallFunction|FindPlayerStartbyTag (Variables|Default|GetCurrentPlayerStartTag)))
  (return _playerstart))

(fn GetGSR
  (params (Cell :type EWorldCells%20Enum :default "NewEnumerator0") (GSRKey :type Name :default "None"))
  ;[1 1 1] Comment
  (LocalVariables|SetCellLocal Cell)
  (LocalVariables|SetGSRKeyLocal GSRKey)
  ;[1 1 1] Find the entry
  (bind _array_element (Utilities|Array|ForEachLoopwithBreak (Variables|Default|GetGSR) :!label _label)
    (:LoopBody
      (if (and (Utilities|Enum|Equal(Enum) (LocalVariables|GetCellLocal) (.Cell (Utilities|Struct|BreakGSRStruct _array_element))) (Utilities|Name|Equal(Name) (.GSRKey (Utilities|Struct|BreakGSRStruct _array_element)) (LocalVariables|GetGSRKeyLocal)))
        (LocalVariables|SetGSRValueLocal (.GSRValue (Utilities|Struct|BreakGSRStruct _array_element)))
        (goto _label Break)))
    (:Completed
      (return (LocalVariables|GetGSRValueLocal)))))

(fn GetMarkers
  (return (Variables|Default|GetQuestMarkers)))

(fn IsCurrentCheckpoint
  (params (PlayerStart :type Player%20Start%20Object%20Reference))
  (return (Utilities|Name|Equal(Name) (Variables|/Script/Engine.PlayerStart|GetPlayerStartTag PlayerStart) (Variables|Default|GetCurrentPlayerStartTag))))

(fn SetCurrentCheckpoint
  (params (NewPlayerStart :type Player%20Start%20Object%20Reference))
  ;[1 1 1] Save what player start to spawn the player at when the game starts
  (Utilities|IsValid NewPlayerStart
    (:Is%20Valid
      (Variables|Default|SetCurrentPlayerStartTag (Variables|/Script/Engine.PlayerStart|GetPlayerStartTag NewPlayerStart)))
    (:Is%20Not%20Valid
      (Variables|Default|SetCurrentPlayerStartTag "Checkpoint_01")))
  (return true))

(fn SetGSR
  (params (Cell :type EWorldCells%20Enum :default "NewEnumerator0") (GSRKey :type Name :default "None") (GSRValue :type Integer))
  ;[1 1 1] Init
  (LocalVariables|SetCellLocal Cell)
  (LocalVariables|SetGSRKeyLocal GSRKey)
  (LocalVariables|SetGSRValueLocal GSRValue)
  (bind (_array_element _array_index) (Utilities|Array|ForEachLoopwithBreak (Variables|Default|GetGSR) :!label _label)
    (:LoopBody
      ;[1 1 1] Update existing entry
      (if (and (Utilities|Enum|Equal(Enum) (LocalVariables|GetCellLocal) (.Cell (Utilities|Struct|BreakGSRStruct _array_element))) (Utilities|Name|Equal(Name) (.GSRKey (Utilities|Struct|BreakGSRStruct _array_element)) (LocalVariables|GetGSRKeyLocal)))
        (Utilities|Array|SetArrayElem (Variables|Default|GetGSR) _array_index (Utilities|Struct|MakeGSRStruct (LocalVariables|GetCellLocal) (LocalVariables|GetGSRKeyLocal) (LocalVariables|GetGSRValueLocal)) true)
        (LocalVariables|SetFoundEntryLocal true)
        (goto _label Break)))
    (:Completed
      (if (LocalVariables|GetFoundEntryLocal)
        _
        (else
          ;[1 1 1] Create a new entry
          (Utilities|Array|Add (Variables|Default|GetGSR) (Utilities|Struct|MakeGSRStruct (LocalVariables|GetCellLocal) (LocalVariables|GetGSRKeyLocal) (LocalVariables|GetGSRValueLocal)))))
      (return true))))

(fn SetJournal
  (params (QuestName :type Text) (Objective :type Text) (Description :type Text))
  (bind _returnvalue (Game|GetGameMode))
  (bind _asquest_game_mode (Utilities|Casting|CastToQuestGameMode _returnvalue))
  (bind _playerhud (Variables|/Game/Blueprints/Game/QuestGameMode.QuestGameMode_C|GetPlayerHUD _asquest_game_mode))
  (Default|SetJournalText _playerhud QuestName Objective Description)
  (Default|OpenJournal _playerhud)
  (return true))

(fn SetMarker
  (params (Marker :type Quest%20Marker%20Object%20Reference))
  (Utilities|IsValid Marker
    (:Is%20Valid
      (Utilities|Array|AddUnique (Variables|Default|GetQuestMarkers) Marker)
      (return true))
    (:Is%20Not%20Valid
      (return false))))