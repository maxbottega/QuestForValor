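; Game mode for the quest game that sets up the player HUD, respawns at checkpoints and controls music.
; On BeginPlay it creates the HUD, records the level name and binds the Juno character's death and destruction to HUD removal and a delayed level reload.
; ChoosePlayerStart uses the game instance's checkpoint, falling back to the parent choice if invalid.
; Music functions fade the MusicController in or out, with StopMusic always fading to silence.
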(event Custom|PlayerDestroyed
  ;[1 1 1] Player has died, restart the level
  (Widget|RemovefromParent (Variables|Default|GetPlayerHUD))
  (Utilities|FlowControl|Delay 3.0)
  (Game|OpenLevel(byName) (Variables|Default|GetCurrentLevelName)))

(event Custom|PlayerDead
  (params (DeadCharacter :type Quest%20Character%20Object%20Reference))
  ;[1 1 1] Player has died, restart the level
  (Widget|RemovefromParent (Variables|Default|GetPlayerHUD))
  (Utilities|FlowControl|Delay 3.0)
  (Game|OpenLevel(byName) (Variables|Default|GetCurrentLevelName)))

(event EventBeginPlay
  ;[1 1 1] Init vars
  (bind _asquest_character_juno (Utilities|Casting|CastToQuestCharacter_Juno (Game|GetPlayerCharacter 0)))
  (Variables|Default|SetPlayerCharacter _asquest_character_juno)
  ;[1 1 1] Create the player HUD
  (bind _returnvalue (UserInterface|CreateWidget "/Game/UI/UMG/QuestUMG_IngameHUD.QuestUMG_IngameHUD_C" (Game|GetPlayerController 0)))
  (Variables|Default|SetPlayerHUD _returnvalue)
  (UserInterface|Viewport|AddtoViewport (Variables|Default|GetPlayerHUD) 0)
  ;[1 1 1] Player has died, restart the level
  (EventDispatchers|AssignOnCharacterDied (Variables|Default|GetPlayerCharacter) (delegate Custom|PlayerDead))
  (Game|AssignOnDestroyed (Variables|Default|GetPlayerCharacter) (delegate Custom|PlayerDestroyed))
  ;[1 1 1] Set the current level
  (bind _returnvalue_2 (Game|GetCurrentLevelName true))
  (CallFunction|SetCurrentLevel (Utilities|String|StringToName _returnvalue_2)))

(fn ConstructionScript)

(fn ChoosePlayerStart
  (params (Player :type Controller%20Object%20Reference))
  (LocalVariables|SetPlayerLocal Player)
  (bind _currentplayerstart (Class|QuestGameInstanceInterface|GetCurrentCheckpoint(Message) (Game|GetGameInstance)))
  (bind _output_get (LocalVariables|SetChosenPlayerStartLocal _currentplayerstart))
  (Utilities|IsValid _output_get
    (:Is%20Valid
      _)
    (:Is%20Not%20Valid
      (bind _returnvalue (|CallParentFunction (LocalVariables|GetPlayerLocal)))
      (LocalVariables|SetChosenPlayerStartLocal _returnvalue)))
  (return (LocalVariables|GetChosenPlayerStartLocal)))

(fn PlayMusic
  (params (MusicTrack :type Sound%20Base%20Object%20Reference) (FadeInDuration :type Float%20%28single-precision%29) (FadeInVolume :type Float%20%28single-precision%29))
  ;[1 1 1] Init vars
  (LocalVariables|SetMusicTrackLocal MusicTrack)
  (LocalVariables|SetFadeInDurationLocal FadeInDuration)
  (LocalVariables|SetFadeInVolumeLocal FadeInVolume)
  ;[1 1 1] Set the music track and then fade it in
  (Audio|Components|Audio|SetSound (Variables|Default|GetMusicController) (LocalVariables|GetMusicTrackLocal))
  (Audio|Components|Audio|FadeIn (Variables|Default|GetMusicController) (LocalVariables|GetFadeInDurationLocal) (LocalVariables|GetFadeInVolumeLocal) 0.0 :!class /Script/Engine.AudioComponent)
  ;[1 1 1] Return
  (return true))

(fn SetCurrentLevel
  (params (LevelName :type Name :default "None"))
  (Variables|Default|SetCurrentLevelName LevelName)
  (return false))

(fn StopMusic
  (params (FadeOutDuration :type Float%20%28single-precision%29) (FadeOutVolume :type Float%20%28single-precision%29))
  ;[1 1 1] Init vars
  (LocalVariables|SetFadeOutDurationLocal FadeOutDuration)
  (LocalVariables|SetFadeVolumeLevelLocal 0.0)
  ;[1 1 1] Fade out based on user settings
  (Audio|Components|Audio|FadeOut (Variables|Default|GetMusicController) (LocalVariables|GetFadeOutDurationLocal) (LocalVariables|GetFadeVolumeLevelLocal) :!class /Script/Engine.AudioComponent)
  ;[1 1 1] Return
  (return true))