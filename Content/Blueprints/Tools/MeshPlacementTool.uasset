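; Editor placement tool Blueprint that builds a straight run of modular static meshes from the actor toward MeshEndPoint.
; Its Construction Script adds a component every MeshLength along MeshBase's X axis, with count derived from that vector's length.
; Optional start and end meshes cap the run, falling back to the body mesh, each type with its own rotation.
; A look-at rotation aims MeshBase along the vector, keeping actor roll.
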(fn ConstructionScript
  (bind _returnvalue (Transformation|GetActorLocation))
  (bind _meshendpoint (Variables|MeshPlacement|GetMeshEndPoint))
  (bind _meshlength (Variables|MeshPlacement|GetMeshLength))
  (bind _meshlength_2 (Variables|MeshPlacement|GetMeshLength))
  (bind _meshlength_3 (Variables|MeshPlacement|GetMeshLength))
  (bind _returnvalue_2 (+ _returnvalue _meshendpoint))
  (bind _returnvalue_3 (Math|Rotator|FindLookatRotation _returnvalue _returnvalue_2))
  (bind (_pitch _yaw) (Class|KismetMathLibrary|BreakRot _returnvalue_3))
  ;[1 1 1] Check if we have meshes supplied for the start and end
  (Variables|MeshPlacement|SetHasMeshStart (Utilities|IsValid (Variables|MeshPlacement|GetMeshStart)))
  (Variables|MeshPlacement|SetHasMeshEnd (Utilities|IsValid (Variables|MeshPlacement|GetMeshEnd)))
  ;[1 1 1] Set the base mesh
  (if (Variables|MeshPlacement|GetHasMeshStart)
    (Components|StaticMesh|SetStaticMesh (Variables|Default|GetMeshFirstStart) (Variables|MeshPlacement|GetMeshStart))
    (else
      (Components|StaticMesh|SetStaticMesh (Variables|Default|GetMeshFirstStart) (Variables|MeshPlacement|GetMeshBody))))
  ;[1 1 1] Make sure the vector is not zero'd out
  (if (Math|Vector|NotEqual(Vector) (Variables|MeshPlacement|GetMeshEndPoint) "0, 0, 0" 0.0001)
    ;[1 1 1] Iterate through the distance
    (bind _output_get (Variables|MeshPlacement|SetNumberOfInstances (Math|Float|Floor (/ (Math|Vector|VectorLength (Variables|MeshPlacement|GetMeshEndPoint)) (Variables|MeshPlacement|GetMeshLength)))))
    (for _index (range 0 _output_get)
      (Variables|MeshPlacement|SetCurrentIndex _index)
      ;[1 1 1] Figure out what index we are on
      (if (== (Variables|MeshPlacement|GetCurrentIndex) 0)
        (Variables|MeshPlacement|SetMeshInstanceXPlacement (+ (* (Variables|MeshPlacement|GetCurrentIndex) _meshlength) _meshlength))
        (bind _returnvalue_4 (AddComponent|AddStaticMeshComponent true :!label _label))
        (bind _output_get_2 (Variables|Default|SetMeshInstance _returnvalue_4))
        (Components|StaticMesh|SetStaticMesh _output_get_2 (Variables|MeshPlacement|GetMeshBody))
        (Class|SceneComponent|Attachto (Variables|Default|GetMeshInstance) (Variables|Default|GetMeshBase) "None" "KeepRelativeOffset" true)
        (Transformation|SetRelativeLocation (Variables|Default|GetMeshInstance) (Math|Vector|MakeVector (Variables|MeshPlacement|GetMeshInstanceXPlacement) 0.0 0.0) false)
        (Transformation|SetRelativeRotation (Variables|Default|GetMeshInstance) (Variables|MeshPlacement|GetMeshBodyRotation) false)
        (elif (not (== (Variables|MeshPlacement|GetCurrentIndex) (Variables|MeshPlacement|GetNumberOfInstances)))
          (Variables|MeshPlacement|SetMeshInstanceXPlacement (+ (* (Variables|MeshPlacement|GetCurrentIndex) _meshlength_3) _meshlength_3) :!label _label_2)
          (goto _label)
          (elif (not (Variables|MeshPlacement|GetHasMeshEnd))
            (goto _label_2)
            (else
              ;[1 1 1] Last mesh to be placed
              (Variables|MeshPlacement|SetMeshInstanceXPlacement (+ (* (Variables|MeshPlacement|GetCurrentIndex) _meshlength_2) _meshlength_2))
              (bind _returnvalue_5 (AddComponent|AddStaticMeshComponent true))
              (bind _output_get_3 (Variables|Default|SetMeshInstance _returnvalue_5))
              (Components|StaticMesh|SetStaticMesh _output_get_3 (Variables|MeshPlacement|GetMeshEnd))
              (Class|SceneComponent|Attachto (Variables|Default|GetMeshInstance) (Variables|Default|GetMeshBase) "None" "KeepRelativeOffset" true)
              (Transformation|SetRelativeLocation (Variables|Default|GetMeshInstance) (Math|Vector|MakeVector (Variables|MeshPlacement|GetMeshInstanceXPlacement) 0.0 0.0) false)
              (Transformation|SetRelativeRotation (Variables|Default|GetMeshInstance) (Variables|MeshPlacement|GetMeshEndRotation) false))))))
    ;[1 1 1] Set rotation based on look at rotation
    (Transformation|SetWorldRotation (Variables|Default|GetMeshBase) (Class|KismetMathLibrary|MakeRot _pitch _yaw (.roll (Transformation|GetActorRotation))) false)
    (if (Variables|MeshPlacement|GetHasMeshStart)
      (Transformation|SetRelativeRotation (Variables|Default|GetMeshFirstStart) (Variables|MeshPlacement|GetMeshStartRotation) false)
      (else
        (Transformation|SetRelativeRotation (Variables|Default|GetMeshFirstStart) (Variables|MeshPlacement|GetMeshBodyRotation) false)))))