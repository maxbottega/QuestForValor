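; Editor tool actor that lays out a row of static meshes from an array for side-by-side preview, each labeled with index and name.
; The construction script snaps the actor to traced ground, then spawns evenly spaced mesh and text components along a line to a target end point.
; Per-mesh rotation and offset arrays adjust placement, and bounds-based scaling enlarges smaller meshes more.
; The Origin component finally rotates toward the end point.
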(event EventBeginPlay)

(event Collision|EventActorBeginOverlap
  (params (OtherActor :type Actor%20Object%20Reference)))

(event EventTick
  (params (DeltaSeconds :type Float%20%28single-precision%29)))

(fn ConstructionScript
  (bind _returnvalue (Transformation|GetActorLocation))
  (bind _returnvalue_2 (Transformation|GetActorLocation))
  (bind _returnvalue_3 (Transformation|GetActorLocation))
  ;[0.3865 1 0.4906] Reset location/rotation and set distance between meshes
  (Transformation|SetActorRotation "0, 0, 0")
  (bind _outhit (Collision|LineTraceForObjects (+ _returnvalue_2 "0, 0,600.000000") _returnvalue_2 (Utilities|Array|MakeArray "ObjectTypeQuery1") true 0 "ForDuration" true "(R=1.000000,G=0.000000,B=0.000000,A=1.000000)" "(R=0.000000,G=1.000000,B=0.000000,A=1.000000)" 1e+01))
  (Transformation|SetActorLocation (Math|Vector|MakeVector (.x _returnvalue) (.y _returnvalue) (+ (.z (.impactpoint _outhit)) 5e+01)) false false)
  (Variables|CustomParameters|Setv_meshEndPoint (Math|Vector|MakeVector (.x (Variables|CustomParameters|Getv_meshEndPoint)) (.y (Variables|CustomParameters|Getv_meshEndPoint)) 0.0))
  (Variables|CustomParameters|Setv_meshesLength (+ (* 2 (.SphereRadius (Collision|GetComponentBounds (Variables|Default|GetStaticMesh)))) (Variables|CustomParameters|Getv_distance)))
  ;[0.3865 1 0.4906] Make sure the vector is not zero'd out
  (if (Math|Vector|NotEqual(Vector) (Variables|CustomParameters|Getv_meshEndPoint) "0, 0, 0" 0.0001)
    ;[0.3865 1 0.4906] Iterate through the distance
    (Variables|CustomParameters|Setv_numberOfInstances (+ (Math|Float|Floor (/ (Math|Vector|VectorLength (Variables|CustomParameters|Getv_meshEndPoint)) (Variables|CustomParameters|Getv_meshesLength))) 1))
    (for _index (range 0 (Math|Float|Floor (/ (Math|Vector|VectorLength (Variables|CustomParameters|Getv_meshEndPoint)) (Variables|CustomParameters|Getv_meshesLength))))
      (Variables|CustomParameters|Setv_currentIndex _index)
      ;[0.3865 1 0.4906] Set where the new mesh is going to be placed
      (Variables|CustomParameters|Setv_meshInstanceXPlacement (* (Variables|CustomParameters|Getv_currentIndex) (Variables|CustomParameters|Getv_meshesLength)))
      ;[0.3865 1 0.4906] Add new Scene component to the actor
      (bind _returnvalue_4 (AddComponent|AddSceneComponent true))
      (bind _output_get (Variables|Default|Setv_sceneComponent _returnvalue_4))
      (Transformation|AttachComponentToComponent _output_get (Variables|Default|GetOrigin) "None" "KeepRelative" "KeepRelative" "KeepRelative" true)
      (Transformation|SetRelativeLocation _output_get (Math|Vector|MakeVector (Variables|CustomParameters|Getv_meshInstanceXPlacement) 0.0 0.0) false false)
      ;[0.3865 1 0.4906] Attach mesh and text to MeshBase, then set their location
      (bind _returnvalue_5 (AddComponent|AddStaticMeshComponent true))
      (Transformation|AttachComponentToComponent _returnvalue_5 _output_get "None" "KeepRelative" "KeepRelative" "KeepRelative" true)
      (Components|StaticMesh|SetStaticMesh _returnvalue_5 (Utilities|Array|Get(acopy) (Variables|CustomParameters|Getv_staticMesh) (Variables|CustomParameters|Getv_currentIndex)))
      (Transformation|AddRelativeRotation _returnvalue_5 (Utilities|Array|Get(acopy) (Variables|CustomParameters|Getv_meshStartRotation) (Variables|CustomParameters|Getv_currentIndex)) false false)
      (Transformation|AddLocalOffset _returnvalue_5 (Math|Vector|MakeVector (* -1 (.y (Utilities|Array|Get(acopy) (Variables|CustomParameters|Getv_manualLocation) (Variables|CustomParameters|Getv_currentIndex)))) (.x (Utilities|Array|Get(acopy) (Variables|CustomParameters|Getv_manualLocation) (Variables|CustomParameters|Getv_currentIndex))) (.z (Utilities|Array|Get(acopy) (Variables|CustomParameters|Getv_manualLocation) (Variables|CustomParameters|Getv_currentIndex)))) false true)
      (Transformation|SetWorldScale3D _returnvalue_5 (Math|Vector|MakeVector (Math|Float|SelectFloat (Math|Float|MapRangeClamped (* (.SphereRadius (Collision|GetComponentBounds _returnvalue_5)) 2.0) 0.0 1.2e+03 4.0 0.0) (Math|Float|MapRangeClamped (* (.SphereRadius (Collision|GetComponentBounds _returnvalue_5)) 2.0) 0.0 1e+02 12.0 4.0) (> (* (.SphereRadius (Collision|GetComponentBounds _returnvalue_5)) 2.0) 1e+02)) (Math|Float|SelectFloat (Math|Float|MapRangeClamped (* (.SphereRadius (Collision|GetComponentBounds _returnvalue_5)) 2.0) 0.0 1.2e+03 4.0 0.0) (Math|Float|MapRangeClamped (* (.SphereRadius (Collision|GetComponentBounds _returnvalue_5)) 2.0) 0.0 1e+02 12.0 4.0) (> (* (.SphereRadius (Collision|GetComponentBounds _returnvalue_5)) 2.0) 1e+02)) (Math|Float|SelectFloat (Math|Float|MapRangeClamped (* (.SphereRadius (Collision|GetComponentBounds _returnvalue_5)) 2.0) 0.0 1.2e+03 4.0 0.0) (Math|Float|MapRangeClamped (* (.SphereRadius (Collision|GetComponentBounds _returnvalue_5)) 2.0) 0.0 1e+02 12.0 4.0) (> (* (.SphereRadius (Collision|GetComponentBounds _returnvalue_5)) 2.0) 1e+02))))
      (bind _returnvalue_6 (AddComponent|AddTextRenderComponent true (Math|Transform|MakeTransform "0,0.000000,1.000000" "90.000000, 0,-90.000000" "1,1,1")))
      (Transformation|AttachComponentToComponent _returnvalue_6 (Variables|Default|Getv_sceneComponent) "None" "SnapToTarget" "KeepRelative" "KeepWorld" true)
      (Transformation|AddWorldOffset _returnvalue_6 "0.000000,250.000000,0.000000" false true)
      (Rendering|Components|TextRender|SetText _returnvalue_6 (Utilities|Text|ToText(String) (Utilities|String|Append "[" (Utilities|String|ToString(Integer) (Variables|CustomParameters|Getv_currentIndex)) "] <br>" (Utilities|GetDisplayName (Utilities|Array|Get(acopy) (Variables|CustomParameters|Getv_staticMesh) (Variables|CustomParameters|Getv_currentIndex))))))
      (Rendering|Components|TextRender|SetWorldSize _returnvalue_6 (Variables|CustomParameters|Getv_textSize)))
    ;[0.3865 1 0.4906] Set rotation based on the location of the last mesh added
    (Transformation|SetWorldRotation (Variables|Default|GetOrigin) (Math|Rotator|FindLookatRotation _returnvalue_3 (+ _returnvalue_3 (Variables|CustomParameters|Getv_meshEndPoint))) false false)))