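; Editor tool actor that previews materials on a row of labeled meshes, built entirely in the Construction Script.
; It zeroes its rotation, traces down to sit on the surface below, and flattens the end point.
; The end-point distance, mesh bounds and gap set the instance count, each taking the next array material and a text label with its name.
; The Origin component then rotates to aim the row at the end point.
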(event EventBeginPlay)

(event Collision|EventActorBeginOverlap
  (params (OtherActor :type Actor%20Object%20Reference)))

(event EventTick
  (params (DeltaSeconds :type Float%20%28single-precision%29)))

(fn ConstructionScript
  (bind _returnvalue (Transformation|GetActorLocation))
  (bind _returnvalue_2 (Transformation|GetActorLocation))
  (bind _returnvalue_3 (Transformation|GetActorLocation))
  ;[0.3865 1 0.4906] Reset location/rotation and set distance between meshes
  (Transformation|SetActorRotation "0, 0, 0")
  (bind _outhit (Collision|LineTraceForObjects (+ _returnvalue_2 "0, 0,600.000000") _returnvalue_2 (Utilities|Array|MakeArray "ObjectTypeQuery1" "ObjectTypeQuery2") false 0 "None"))
  (Transformation|SetActorLocation (Math|Vector|MakeVector (.x _returnvalue) (.y _returnvalue) (.z (.impactpoint _outhit))) false false)
  (Variables|CustomParameters|Setv_meshEndPoint (Math|Vector|MakeVector (.x (Variables|CustomParameters|Getv_meshEndPoint)) (.y (Variables|CustomParameters|Getv_meshEndPoint)) 0.0))
  (Variables|CustomParameters|Setv_meshesLength (+ (* 2 (.x (.Max (Components|StaticMesh|GetLocalBounds (Variables|Default|GetStaticMesh))))) (Variables|CustomParameters|Getv_distance)))
  ;[0.3865 1 0.4906] Make sure the vector is not zero'd out
  (if (Math|Vector|NotEqual(Vector) (Variables|CustomParameters|Getv_meshEndPoint) "0, 0, 0" 0.0001)
    ;[0.3865 1 0.4906] Iterate through the distance
    (Variables|CustomParameters|Setv_numberOfInstances (+ (Math|Float|Floor (/ (Math|Vector|VectorLength (Variables|CustomParameters|Getv_meshEndPoint)) (Variables|CustomParameters|Getv_meshesLength))) 1))
    (for _index (range 0 (Math|Float|Floor (/ (Math|Vector|VectorLength (Variables|CustomParameters|Getv_meshEndPoint)) (Variables|CustomParameters|Getv_meshesLength))))
      (Variables|CustomParameters|Setv_currentIndex _index)
      ;[0.3865 1 0.4906] Set where the new mesh is going to be placed
      (Variables|CustomParameters|Setv_meshInstanceXPlacement (* (Variables|CustomParameters|Getv_currentIndex) (Variables|CustomParameters|Getv_meshesLength)))
      ;[0.3865 1 0.4906] Add new mesh component to the actor
      (bind _returnvalue_4 (AddComponent|AddStaticMeshComponent true))
      ;[0.3865 1 0.4906] Attach mesh and text to MeshBase, then set their location
      (Transformation|AttachComponentToComponent _returnvalue_4 (Variables|Default|GetOrigin) "None" "KeepRelative" "KeepRelative" "KeepRelative" true)
      (Transformation|SetRelativeLocation _returnvalue_4 (Math|Vector|MakeVector (Variables|CustomParameters|Getv_meshInstanceXPlacement) 0.0 0.0) false false)
      (Transformation|SetRelativeRotation _returnvalue_4 (Variables|CustomParameters|Getv_meshStartRotation) false false)
      (Rendering|Material|SetMaterial _returnvalue_4 0 (Utilities|Array|Get(acopy) (Variables|CustomParameters|Getv_material) (Variables|CustomParameters|Getv_currentIndex)))
      (bind _returnvalue_5 (AddComponent|AddTextRenderComponent false (Math|Transform|MakeTransform "0,150.000000,1.000000" "90.000000, 0,-90.000000" "1,1,1")))
      (Transformation|AttachComponentToComponent _returnvalue_5 _returnvalue_4 "None" "KeepRelative" "KeepRelative" "KeepRelative" true)
      (Rendering|Components|TextRender|SetText _returnvalue_5 (Utilities|Text|ToText(String) (Utilities|GetDisplayName (Utilities|Array|Get(acopy) (Variables|CustomParameters|Getv_material) (Variables|CustomParameters|Getv_currentIndex))))))
    ;[0.3865 1 0.4906] Set rotation based on the location of the last mesh added
    (Transformation|SetWorldRotation (Variables|Default|GetOrigin) (Math|Rotator|FindLookatRotation _returnvalue_3 (+ _returnvalue_3 (Variables|CustomParameters|Getv_meshEndPoint))) false false)))